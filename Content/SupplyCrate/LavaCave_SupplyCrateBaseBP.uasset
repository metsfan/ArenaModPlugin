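; Base Blueprint for a Lava Cave supply crate that players must unlock with a timed hold interaction.
; While locked, it replaces the multi-use entries with an unlock prompt, offering the timed Unlock action only if the arena-mod player pawn was not recently damaged.
; Using that action sets Unlocked and calls ClientUnlock to set it again; other uses go to the parent, and unlocked crates keep incoming entries unchanged.
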(event Custom|ClientUnlock
  (Variables|Default|SetUnlocked true false))

(fn ConstructionScript)

(fn BPTryMultiUse
  (params (ForPC :type Player%20Controller%20Object%20Reference) (UseIndex :type Integer))
  (if (== UseIndex 987)
    (Variables|Default|SetUnlocked true false)
    (CallFunction|ClientUnlock)
    (else
      (bind _returnvalue (|CallParentFunction ForPC UseIndex))))
  (return _returnvalue))

(fn BPGetMultiUseEntries
  (params (ForPC :type Player%20Controller%20Object%20Reference) (MultiUseEntries :type Array%20of%20Multi%20Use%20Entry%20Structures))
  (bind _unlocktime (Variables|Default|GetUnlockTime))
  (Utilities|FlowControl|Sequence
    (:then_0
      (if (not (Variables|Default|GetUnlocked))
        (Utilities|Array|Clear MultiUseEntries)
        (Utilities|Array|Add MultiUseEntries (Utilities|Struct|MakeMultiUseEntry 0 "[Hold E to Unlock]" 0 10 true))
        (bind _asplayer_pawn_test_child_arena_mod (Utilities|Casting|CastToPlayerPawnTest_Child_ArenaMod (Pawn|GetControlledPawn ForPC)))
        (if (not (Variables|/ArenaMod/PlayerPawnTest_Child_ArenaMod.PlayerPawnTest_Child_ArenaMod_C|GetRecentlyDamaged _asplayer_pawn_test_child_arena_mod))
          (Utilities|Array|Add MultiUseEntries (Utilities|Struct|MakeMultiUseEntry 0 "Unlock" 987 1 false false false false false false false false false false false false false false 0 false 0 "(B=175,G=175,R=175,A=255)" "(B=255,G=255,R=255,A=255)" _unlocktime _unlocktime)))))
    (:then_1
      (return MultiUseEntries))))