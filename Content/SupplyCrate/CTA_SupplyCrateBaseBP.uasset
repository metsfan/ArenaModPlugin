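; Base supply crate, a container players must hold-to-unlock, with that option withheld from recently damaged arena pawns.
; Multi-use overrides offer the timed unlock entry and set the unlocked state.
; BeginPlay creates cosmetic spawn-in effects off dedicated servers, which the FinishedSpawn RepNotify shuts down, alongside empty spawn hooks.
; A randomly staggered looping timer mirrors the day cycle manager's hide flag onto crate, emitter and child actor.
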(event Custom|DestroyEmitter
  (Actor|DestroyActor (Variables|Default|GetSpawnInLocationEmitterInstance)))

(event Custom|ClientUnlock
  (Variables|Default|SetUnlocked true false))

(event Custom|CheckHiding
  (bind _returnvalue (Class|PrimalGlobals|GetDayCycleManager (Class|PrimalActor|GetWorld)))
  (if (Math|Boolean|NotEqual(Boolean) (Variables|/Script/ShooterGame.DayCycleManager|GetbHideSupplyCrates _returnvalue) (Variables|Default|GetbHiddenStuff))
    (Variables|Default|SetbHiddenStuff (Variables|/Script/ShooterGame.DayCycleManager|GetbHideSupplyCrates _returnvalue))
    (Rendering|SetActorHiddenInGame (Variables|Default|GetSpawnInLocationEmitterInstance) (Variables|/Script/ShooterGame.DayCycleManager|GetbHideSupplyCrates _returnvalue))
    (Rendering|SetActorHiddenInGame (Variables|/Script/ShooterGame.DayCycleManager|GetbHideSupplyCrates _returnvalue))
    (bind _aschild_actor_component (Utilities|Casting|CastToChildActorComponent (Actor|GetComponentbyClass "/Script/Engine.ChildActorComponent")))
    (Rendering|SetActorHiddenInGame (Variables|/Script/Engine.ChildActorComponent|GetChildActor _aschild_actor_component) (Variables|/Script/ShooterGame.DayCycleManager|GetbHideSupplyCrates _returnvalue))
    (if (not (Variables|/Script/Engine.Actor|GetbHidden (Variables|/Script/Engine.ChildActorComponent|GetChildActor _aschild_actor_component)))
      (if (Variables|Default|GetbContainerActivated)
        (bind _asemitter (Utilities|Casting|CastToEmitter (Variables|/Script/Engine.ChildActorComponent|GetChildActor _aschild_actor_component)))
        (Components|Activation|Activate _asemitter true)))))

(event Custom|OnSpawningIn)

(event Custom|OnCompletedSpawning)

(event EventBeginPlay
  (Utilities|FlowControl|Sequence
    (:then_0
      (Networking|SwitchHasAuthority
        (:Authority
          (Variables|Default|SetInitialLoc (Transformation|GetActorLocation) false)
          (Variables|Default|SetInitialRot (Transformation|GetActorRotation) false))
        (:Remote
          _))
      (Class|Actor|AttachRootComponenttoActor 0 "None" "SnapToTarget" true)
      (if (not (Variables|Default|GetbFinishedSpawn))
        (Utilities|FlowControl|Sequence
          (:then_0
            (if (not (Networking|IsDedicatedServer))
              (bind _returnvalue (AddComponent|AddParticleSystemComponent false (Math|Transform|MakeTransform "0, 0, 0" "0, 0, 0" "10.000000,10.000000,10.000000")))
              (Effects|Components|ParticleSystem|SetTemplate _returnvalue (Variables|Default|GetSpawnInAttachedParticle))
              (Variables|Default|SetSpawnInAttachedPSC _returnvalue)
              (Transformation|SetRelativeScale3D _returnvalue (Variables|Default|GetSpawnInAttachedParticleScale))
              (bind _returnvalue_2 (Game|SpawnActorfromClass (Variables|Default|GetSpawnInLocationEffect) (Math|Conversions|ToTransform(Vector) "0, 0, 0") "AdjustIfPossibleButDontSpawnIfColliding" "SelectDefaultAtRuntime" 0 0))
              (Class|Actor|AttachRootComponenttoActor _returnvalue_2 0 "None" "SnapToTarget" true)
              (Variables|Default|SetSpawnInLocationEmitterInstance _returnvalue_2)))
          (:then_1
            (CallFunction|OnSpawningin)))))
    (:then_1
      (Networking|SwitchHasAuthority))
    (:then_2
      (if (not (Networking|IsDedicatedServer))
        (Utilities|Time|SetTimerbyFunctionName 0 "CheckHiding" (Math|Random|RandomFloatinRange 3.0 8.0) true)
        (Class|KismetSystemLibrary|SetTimerforNextTick 0 "CheckHiding" false)
        (CallFunction|CheckHiding)))))

(event EventDestroyed
  (Utilities|FlowControl|Sequence
    (:then_0
      (Actor|DestroyActor)
      (Actor|DestroyActor))
    (:then_1
      (Actor|DestroyActor (Variables|Default|GetSpawnInLocationEmitterInstance)))))

(fn ConstructionScript)

(fn OnRepBFinishedSpawn
  (Components|Activation|Deactivate (Variables|Default|GetSpawnInAttachedPSC))
  (CallFunction|OnCompletedSpawning)
  (if (not (Networking|IsDedicatedServer))
    (bind _asemitter (Utilities|Casting|CastToEmitter (Variables|Default|GetSpawnInLocationEmitterInstance)))
    (Components|Activation|Deactivate _asemitter)
    (Utilities|Time|SetTimerbyFunctionName 0 "DestroyEmitter" 3.0)))

(fn BPGetMultiUseEntries
  (params (ForPC :type Player%20Controller%20Object%20Reference) (MultiUseEntries :type Array%20of%20Multi%20Use%20Entry%20Structures))
  (Utilities|FlowControl|Sequence
    (:then_0
      (if (not (Variables|Default|GetUnlocked))
        (Utilities|Array|Clear MultiUseEntries)
        (Utilities|Array|Add MultiUseEntries (Utilities|Struct|MakeMultiUseEntry 0 "[Hold E to Unlock]" 0 10 true))
        (bind _asplayer_pawn_test_child_arena_mod (Utilities|Casting|CastToPlayerPawnTest_Child_ArenaMod (Pawn|GetControlledPawn ForPC)))
        (if (not (Variables|/ArenaMod/PlayerPawnTest_Child_ArenaMod.PlayerPawnTest_Child_ArenaMod_C|GetRecentlyDamaged _asplayer_pawn_test_child_arena_mod))
          (Utilities|Array|Add MultiUseEntries (Utilities|Struct|MakeMultiUseEntry 0 "Unlock" 987 1 false false false false false false false false false false false false false false 0 false 0 "(B=175,G=175,R=175,A=255)" "(B=255,G=255,R=255,A=255)" 3.0 3.0)))))
    (:then_1
      (return MultiUseEntries))))

(fn BPTryMultiUse
  (params (ForPC :type Player%20Controller%20Object%20Reference) (UseIndex :type Integer))
  (if (== UseIndex 987)
    (Variables|Default|SetUnlocked true false)
    (CallFunction|ClientUnlock)
    (else
      (bind _returnvalue (|CallParentFunction ForPC UseIndex))))
  (return _returnvalue))