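; BP_ArenaStructureBuilder places the arena mod's structures, a replicator and a vault storage box, at hardcoded world transforms.
; Shortly after BeginPlay, CreateStructures runs on the server only and calls CreateStructureOfClass for each structure.
; That helper destroys every existing actor of the class before spawning one, adjusting for collisions or skipping the spawn if blocked.
; Unconnected leftover nodes hold a game mode server check and teleporter and chibi vault placements.
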(event Custom|CreateStructures
  (if (Networking|IsServer)
    (Utilities|FlowControl|Sequence
      (:then_0
        (CallFunction|CreateStructureOfClass "/ArenaMod/Structures/StorageBox_ArenaReplicator.StorageBox_ArenaReplicator_C" (Math|Transform|MakeTransform "0, 0, 0"))
        (CallFunction|CreateStructureOfClass "/ArenaMod/Structures/StorageBox_ArenaVault.StorageBox_ArenaVault_C" (Math|Transform|MakeTransform "500.000000,500.000000,0.000000"))))))

(event EventBeginPlay
  (Utilities|FlowControl|Delay 0 0.5)
  (CallFunction|CreateStructures))

(fn ConstructionScript)

(fn CreateStructureOfClass
  (params (Class :type Actor%20Class%20Reference) (Transform :type Transform))
  (Utilities|FlowControl|Sequence
    (:then_0
      (bind _outactors (Actor|GetAllActorsOfClass 0 Class))
      (for _array_element _outactors
        (Actor|DestroyActor _array_element)))
    (:then_1
      (Game|SpawnActorfromClass Class Transform "AdjustIfPossibleButDontSpawnIfColliding" "SelectDefaultAtRuntime" 0 0))))