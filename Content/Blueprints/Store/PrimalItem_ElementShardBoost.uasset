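; PrimalItem_ElementShardBoost is a craftable store item that grants or extends a timed element shard bonus for the player who owns it.
; On craft, it adds the Buff_ElementShardBonus buff to the ArenaMod player pawn if that buff is absent.
; It then extends the bonus expiry on the player controller by the boost duration, flagging whether the buff is new, sets the bonus multiplier and forces a net update.
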(fn BPCrafted
  (bind _asplayer_pawn_test_child_arena_mod (Utilities|Casting|CastToPlayerPawnTest_Child_ArenaMod (Variables|Default|GetLastOwnerPlayer)))
  (Utilities|FlowControl|Sequence
    (:then_0
      (LocalVariables|SetNewBuff (not (Class|PrimalCharacter|HasBuff _asplayer_pawn_test_child_arena_mod "/ArenaMod/Blueprints/Store/Buff_ElementShardBonus.Buff_ElementShardBonus_C" false)))
      (if (not (Class|PrimalCharacter|HasBuff _asplayer_pawn_test_child_arena_mod "/ArenaMod/Blueprints/Store/Buff_ElementShardBonus.Buff_ElementShardBonus_C" false))
        (Class|PrimalBuff|StaticAddBuff "/ArenaMod/Blueprints/Store/Buff_ElementShardBonus.Buff_ElementShardBonus_C" _asplayer_pawn_test_child_arena_mod 0 0 false)))
    (:then_1
      (bind _returnvalue (Class|Actor|GetOwnerController _asplayer_pawn_test_child_arena_mod))
      (bind _asplayer_controller_blueprint_arena_mod (Utilities|Casting|CastToPlayerControllerBlueprint_ArenaMod _returnvalue))
      (Default|ExtendElementShardBonusExpiry _asplayer_controller_blueprint_arena_mod (Math|Conversions|ToFloat(Integer) (Variables|Default|GetBoostDuration)) (LocalVariables|GetNewBuff))
      (Variables|/ArenaMod/PlayerControllerBlueprint_ArenaMod.PlayerControllerBlueprint_ArenaMod_C|SetElementShardBonusMultiplier _asplayer_controller_blueprint_arena_mod (Variables|Default|GetBonusMultiplier) false)
      (Networking|ForceNetUpdate _asplayer_controller_blueprint_arena_mod))))