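; Timed status buff for the arena mod's Element Shard bonus, showing its remaining time and ending it on expiry.
; The expiry timestamp lives on the instigator's ArenaMod player controller and is compared to real-world UTC time.
; Throttled tick deactivates the buff once that time passes.
; HUD drawing renders a centered countdown on the buff icon, switching to a smaller font when over a day remains.
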(fn ConstructionScript)

(fn ThrottledTick
  (bind _returnvalue (Class|Actor|GetOwnerController (Variables|Default|GetInstigator)))
  (bind _asplayer_controller_blueprint_arena_mod (Utilities|Casting|CastToPlayerControllerBlueprint_ArenaMod _returnvalue))
  (if (<= (Variables|/ArenaMod/PlayerControllerBlueprint_ArenaMod.PlayerControllerBlueprint_ArenaMod_C|GetElementShardBonusExpiry _asplayer_controller_blueprint_arena_mod) (Class|VictoryCore|GetRealWorldUtcTimeinSeconds))
    (Class|PrimalBuff|BPDeactivate)))

(fn BPDrawBuffStatusHUD
  (params (HUD :type Shooter%20HUD%20Object%20Reference) (XPos :type Float%20%28single-precision%29) (YPos :type Float%20%28single-precision%29) (ScaleMult :type Float%20%28single-precision%29))
  (bind _returnvalue (* 4e+01 ScaleMult))
  (bind _returnvalue_2 (Class|Actor|GetOwnerController (Variables|Default|GetInstigator)))
  (bind _asplayer_controller_blueprint_arena_mod (Utilities|Casting|CastToPlayerControllerBlueprint_ArenaMod _returnvalue_2))
  (Class|Canvas|BPDrawTextCentered (Variables|/Script/Engine.HUD|GetCanvas HUD) (.AsFont (Utilities|Casting|CastToFont (Utilities|SelectObject (Variables|/Script/ShooterGame.ShooterHUD|GetSmallFont HUD) (Variables|/Script/ShooterGame.ShooterHUD|GetNormalFont HUD) (> (Math|Float|Round (Math|Conversions|ToFloat(Integer) (- (Variables|/ArenaMod/PlayerControllerBlueprint_ArenaMod.PlayerControllerBlueprint_ArenaMod_C|GetElementShardBonusExpiry _asplayer_controller_blueprint_arena_mod) (Class|VictoryCore|GetRealWorldUtcTimeinSeconds)))) 86400)))) (Class|VictoryCore|BPFormatasTime (Math|Float|Round (Math|Conversions|ToFloat(Integer) (- (Variables|/ArenaMod/PlayerControllerBlueprint_ArenaMod.PlayerControllerBlueprint_ArenaMod_C|GetElementShardBonusExpiry _asplayer_controller_blueprint_arena_mod) (Class|VictoryCore|GetRealWorldUtcTimeinSeconds)))) false false true) (+ XPos (* 32.0 ScaleMult)) (+ (+ YPos _returnvalue) (* _returnvalue -0.5)) 1.0 1.0 true false))