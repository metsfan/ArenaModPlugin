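; Random chibi item that grants a randomly picked chibi in its place when something tries to add it to an inventory.
; The can-add check loads classes listed by name into the chibi pool, spawns a random pick into the target inventory, sets its flags, then refuses itself.
; The force remote-add hook also spawns a pick, without loading names or setting flags.
; The regular remote-add check always refuses.
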(fn BPForceAllowRemoteAddtoInventory
  (params (toInventory :type Primal%20Inventory%20Component%20Object%20Reference))
  (bind _chibiclasses (Variables|Default|GetChibiClasses))
  (Utilities|FlowControl|Sequence
    (:then_0
      (Class|PrimalItem|AddNewItem (Utilities|Array|Get(acopy) _chibiclasses (Math|Random|RandomIntegerinRange 0 (- (Utilities|Array|Length _chibiclasses) 1))) toInventory false false 0.0 true 0 false 0.0 false 0 0.0 false false false))
    (:then_1
      (return false))))

(fn BPCanAddtoInventory
  (params (toInventory :type Primal%20Inventory%20Component%20Object%20Reference))
  (bind _chibiclasses (Variables|Default|GetChibiClasses))
  (CallFunction|AddNamedChibiClasses)
  (Utilities|FlowControl|Sequence
    (:then_0
      (bind _returnvalue (Class|PrimalItem|AddNewItem (Utilities|Array|Get(acopy) _chibiclasses (Math|Random|RandomIntegerinRange 0 (- (Utilities|Array|Length _chibiclasses) 1))) toInventory false false 0.0 true 0 false 0.0 false 0 0.0 false false false))
      (CallFunction|SetChibiItemFlags _returnvalue))
    (:then_1
      (return false))))

(fn BPAllowRemoteAddtoInventory
  (params (invComp :type Primal%20Inventory%20Component%20Object%20Reference) (ByPC :type Shooter%20Player%20Controller%20Object%20Reference) (bRequestedByPlayer :type Boolean))
  (return false))

(fn AddNamedChibiClasses
  (for _array_element (Variables|Default|GetChibiClassNames)
    (bind _returnvalue (Class|VictoryCore|BPLoadClass _array_element))
    (if (!= _returnvalue 0)
      (bind _asprimal_item (Utilities|Casting|CastToPrimalItemClass _returnvalue))
      (Utilities|Array|Add (Variables|Default|GetChibiClasses) _asprimal_item))))