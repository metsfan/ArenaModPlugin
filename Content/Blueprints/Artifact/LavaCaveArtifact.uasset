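; Lava Cave artifact item that gives a buff to the player who picks it up and cannot be remotely taken from trophy bases.
; Its can-add check has a side effect: it resolves the inventory owner's arena-mod controller, applies Buff_LavaCaveArtifact to the controlled character and sets PreventAdd.
; The check always returns true, even when the controller cast fails.
; Remote removal is refused only for the PrimalInventoryBP_TrophyBase inventory class.
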(fn BPCanAddtoInventory
  (params (toInventory :type Primal%20Inventory%20Component%20Object%20Reference))
  (Utilities|FlowControl|Sequence
    (:then_0
      (bind _returnvalue (Class|Actor|GetOwnerController (Components|GetOwner toInventory)))
      (bind _asplayer_controller_blueprint_arena_mod (Utilities|Casting|CastToPlayerControllerBlueprint_ArenaMod _returnvalue))
      (bind _character (CallFunction|GetControlledCharacter _asplayer_controller_blueprint_arena_mod))
      (Class|PrimalBuff|StaticAddBuff "/ArenaMod/Blueprints/Artifact/Buff_LavaCaveArtifact.Buff_LavaCaveArtifact_C" _character 0 0 false)
      (LocalVariables|SetPreventAdd true))
    (:then_2
      (return true))))

(fn BPAllowRemoteRemovefromInventory
  (params (invComp :type Primal%20Inventory%20Component%20Object%20Reference) (ByPC :type Shooter%20Player%20Controller%20Object%20Reference) (bRequestedByPlayer :type Boolean))
  (return (!= (Utilities|GetClass invComp) "/Game/PrimalEarth/CoreBlueprints/Inventories/PrimalInventoryBP_TrophyBase.PrimalInventoryBP_TrophyBase_C")))