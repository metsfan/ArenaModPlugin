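; Base inventory item for points in the Arena mod's Capture the Artifact mode.
; Its add-to-inventory check currently just returns true.
; Disconnected logic in that check would award the item quantity as points to the receiving player's team through the game manager, then force-remove the item from its owner inventory.
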(fn BPCanAddtoInventory
  (params (toInventory :type Primal%20Inventory%20Component%20Object%20Reference))
  (return true))