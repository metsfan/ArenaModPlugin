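; Craftable resource item for the Capture the Artifact arena mode that rewards the crafter's team with a buff and points.
; On BPCrafted, it resolves the Capture the Artifact game manager and current team from the last owner's player controller.
; It adds the configured buff class to that team, or extends an existing one by that buff's Duration, then awards the configured points.
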(fn BPCrafted
  (bind _buffclass (Variables|Default|GetBuffClass))
  (bind _asctateam_buff (Utilities|Casting|CastToCTATeamBuffClass _buffclass))
  (bind _asplayer_pawn_test_child_arena_mod (Utilities|Casting|CastToPlayerPawnTest_Child_ArenaMod (Variables|Default|GetLastOwnerPlayer)))
  (bind _returnvalue (Class|Actor|GetOwnerController _asplayer_pawn_test_child_arena_mod))
  (bind _asplayer_controller_blueprint_arena_mod (Utilities|Casting|CastToPlayerControllerBlueprint_ArenaMod _returnvalue))
  (bind _gamemanager (Default|GetCurrentGameManager _asplayer_controller_blueprint_arena_mod))
  (bind _asgame_manager_capture_the_artifact (Utilities|Casting|CastToGameManager_CaptureTheArtifact _gamemanager))
  (Utilities|FlowControl|Sequence
    (:then_0
      (bind (_hasbuff _buff) (CallFunction|GetCTATeamBuff _asctateam_buff _asgame_manager_capture_the_artifact (Variables|/ArenaMod/PlayerControllerBlueprint_ArenaMod.PlayerControllerBlueprint_ArenaMod_C|GetCurrentGameTeam _asplayer_controller_blueprint_arena_mod)))
      (if _hasbuff
        (Default|ExtendDuration _buff (Variables|/ArenaMod/GameManager/CTA/TeamBuff/CTATeamBuff.CTATeamBuff_C|GetDuration _buff))
        (else
          (CallFunction|AddCTATeamBuff _asctateam_buff _asgame_manager_capture_the_artifact (Variables|/ArenaMod/PlayerControllerBlueprint_ArenaMod.PlayerControllerBlueprint_ArenaMod_C|GetCurrentGameTeam _asplayer_controller_blueprint_arena_mod)))))
    (:then_1
      (Default|GivePointstoTeam _asgame_manager_capture_the_artifact (Variables|/ArenaMod/PlayerControllerBlueprint_ArenaMod.PlayerControllerBlueprint_ArenaMod_C|GetCurrentGameTeam _asplayer_controller_blueprint_arena_mod) (Variables|Default|GetPoints)))))