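; Arena mod variant of the Tek Armor boots buff that lets the arena's player controller switch the boots' Tek abilities on or off.
; It reads CanUseTekAbilities from the owning player's PlayerControllerBlueprint_ArenaMod, running the parent server tick only when that flag is true.
; CanUseTekAbility combines the parent's result with the same flag, so a failed controller cast also denies the ability.
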(event EventBuffTickServer
  (params (DeltaTime :type Float%20%28single-precision%29))
  (bind _returnvalue (Class|Actor|GetOwnerController (CallFunction|GetRefOwningPlayer)))
  (bind _asplayer_controller_blueprint_arena_mod (Utilities|Casting|CastToPlayerControllerBlueprint_ArenaMod _returnvalue))
  (if (Variables|/ArenaMod/PlayerControllerBlueprint_ArenaMod.PlayerControllerBlueprint_ArenaMod_C|GetCanUseTekAbilities _asplayer_controller_blueprint_arena_mod)
    (|CallParentFunction DeltaTime)))

(fn ConstructionScript
  (|CallParentFunction))

(fn CanUseTekAbility
  (params (bNotifyIfOutOfElement :type Boolean))
  (bind _bresult (|CallParentFunction bNotifyIfOutOfElement))
  (Utilities|FlowControl|Sequence
    (:then_0
      (bind _returnvalue (Class|Actor|GetOwnerController (CallFunction|GetRefOwningPlayer)))
      (bind _asplayer_controller_blueprint_arena_mod (Utilities|Casting|CastToPlayerControllerBlueprint_ArenaMod _returnvalue))
      (LocalVariables|SetRet (Variables|/ArenaMod/PlayerControllerBlueprint_ArenaMod.PlayerControllerBlueprint_ArenaMod_C|GetCanUseTekAbilities _asplayer_controller_blueprint_arena_mod)))
    (:then_1
      (return (and _bresult (LocalVariables|GetRet))))))