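; Arena base buff for grappled characters that decides when a grapple tether should break.
; Its ShouldTetherBreak looks up the reworked Tek armor shirt buff on the tether's GrappleOwner.
; The tether breaks only if that buff is valid and its thruster state differs from the first enum value.
; The character and break-distance inputs are ignored, and the construction script only calls the parent.
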(fn ConstructionScript
  (|CallParentFunction))

(fn ShouldTetherBreak
  (params (ForTether :type Grapple%20Tether%20Structure%20%28by%20ref%29) (ForChar :type Primal%20Character%20Object%20Reference) (OverrideBreakPastDist :type Float%20%28single-precision%29))
  (bind _grappleowner (Utilities|Struct|BreakGrappleTether ForTether))
  (bind _returnvalue (Class|PrimalCharacter|GetBuff _grappleowner "/ArenaMod/Blueprints/Armor/Arena_Buff_TekAArmor_Shirt_Rework.Arena_Buff_TekAArmor_Shirt_Rework_C"))
  (return (and (Utilities|IsValid _returnvalue) (!= (Variables|/Game/PrimalEarth/CoreBlueprints/Buffs/Buff_TekArmor_Shirt_Rework.Buff_TekArmor_Shirt_Rework_C|GetCurrentThrusterState (.AsArena%20Buff%20Tek%20AArmor%20Shirt%20Rework (Utilities|Casting|CastToArena_Buff_TekAArmor_Shirt_Rework _returnvalue))) (Utilities|Enum|LiteralenumE_TekThrusterState "NewEnumerator0")))))