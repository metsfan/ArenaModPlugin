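; Arena variant of the Tek Armor pants buff that adds a further restriction on when the owning player can use Tek abilities.
; The CanUseTekAbility override combines the parent check with a CanUseTekAbilities check on the owning character, and both must pass.
; When that extra check fails, it sends its error to the owner's ShooterPlayerController as a Tek Armor notification, regardless of the NotifyIfOutOfElement flag.
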(fn ConstructionScript
  (|CallParentFunction))

(fn CanUseTekAbility
  (params (bNotifyIfOutOfElement :type Boolean))
  (bind _bresult (|CallParentFunction bNotifyIfOutOfElement))
  (Utilities|FlowControl|Sequence
    (:then_0
      (bind (_canuse _error) (CallFunction|CanUseTekAbilities (CallFunction|GetRefOwningPlayer)))
      (Utilities|FlowControl|Sequence
        (:then_0
          (LocalVariables|SetRet _canuse))
        (:then_1
          (if (not _canuse)
            (bind _returnvalue (Class|Actor|GetOwnerController))
            (Class|ShooterPlayerController|ClientServerNotificationSingle (.AsShooter%20Player%20Controller (Utilities|Casting|CastToShooterPlayerController _returnvalue)) _error (Variables|Default|GetTekArmorMessage_Color) (Variables|Default|GetTekArmorMessage_DisplayScale) (Variables|Default|GetTekArmorMessage_DisplayTime) (Variables|Default|GetTekArmorIcon))))))
    (:then_1
      (return (and _bresult (LocalVariables|GetRet))))))