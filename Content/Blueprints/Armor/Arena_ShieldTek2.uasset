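; Arena mod Tek shield item that spends element and durability to reflect incoming fire back at attackers.
; Instant-hit damage is zeroed on the server and re-fired through the attacker's weapon from the wearer, with random spread.
; Blocked projectiles are redirected toward their causer or instigator at unchanged speed, or reversed without one.
; Hit effects replicate through item exec commands, clip ammo toggles emissive glow, and colors come from the Arena game state.
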(fn HandleShieldDamageBlocking
  (params (ForShooterCharacter :type Shooter%20Character%20Object%20Reference) (DamageIn :type Float%20%28single-precision%29) (DamageEvent :type Damage%20Event%20Structure%20%28by%20ref%29) (EventInstigator :type Controller%20Object%20Reference) (DamageCauser :type Actor%20Object%20Reference) (HitPoint :type Vector :default "0, 0, 0"))
  (bind _damagetypeclass (Utilities|Struct|BreakDamageEvent DamageEvent))
  (bind _returnvalue (Transformation|GetActorLocation ForShooterCharacter))
  (LocalVariables|SetDamageOut DamageIn)
  (Utilities|FlowControl|Sequence
    (:then_0
      (if (Networking|IsServer ForShooterCharacter)
        (if (!= _damagetypeclass 0)
          (bind _returnvalue_2 (Class|VictoryCore|GetClassDefaultObject _damagetypeclass))
          (bind _asshooter_damage_type (Utilities|Casting|CastToShooterDamageType _returnvalue_2))
          (if (Variables|/Script/ShooterGame.ShooterDamageType|GetbIsInstantDamage _asshooter_damage_type)
            (bind _candecrease (CallFunction|CanElementDecrease 1 false))
            (if _candecrease
              (Utilities|FlowControl|Sequence
                (:then_0
                  (bind _asshooter_character (Utilities|Casting|CastToShooterCharacter DamageCauser))
                  (bind _asshooter_weapon_instant (Utilities|Casting|CastToShooterWeapon_Instant (Variables|/Script/ShooterGame.ShooterCharacter|GetCurrentWeapon _asshooter_character)))
                  (Class|PrimalCharacter|NetForceUpdateAimedCharacters ForShooterCharacter _returnvalue (Transformation|GetActorLocation _asshooter_character) 0 false 2e+03)
                  (bind (_outhit _returnvalue_3) (Collision|LineTraceByChannel ForShooterCharacter _returnvalue (+ (* (Math|Vector|RotateVector (Math|Vector|Normalize (- (Transformation|GetSocketLocation (Variables|/Script/Engine.Character|GetMesh _asshooter_character) "FloatingHUDSocketRagdoll") _returnvalue)) (Math|Rotator|MakeRotator 0.0 (Math|Random|RandomFloatinRange -1.45 1.45) (Math|Random|RandomFloatinRange -1.45 1.45))) (.WeaponRange (Utilities|Struct|BreakInstantWeaponData (Variables|/Script/ShooterGame.ShooterWeapon|GetInstantConfig _asshooter_weapon_instant)))) _returnvalue) "TraceTypeQuery2" false (Utilities|Array|MakeArray ForShooterCharacter) "None"))
                  (if _returnvalue_3
                    (Class|ShooterWeaponInstant|ServerForceShot _asshooter_weapon_instant _outhit (+ (* (Math|Vector|RotateVector (Math|Vector|Normalize (- (Transformation|GetSocketLocation (Variables|/Script/Engine.Character|GetMesh _asshooter_character) "FloatingHUDSocketRagdoll") _returnvalue)) (Math|Rotator|MakeRotator 0.0 (Math|Random|RandomFloatinRange -1.45 1.45) (Math|Random|RandomFloatinRange -1.45 1.45))) 15.0) _returnvalue) (.Location (Collision|BreakHitResult _outhit)))
                    (else
                      (Class|ShooterWeaponInstant|ServerForceShot _asshooter_weapon_instant (LocalVariables|GetNullHitResult) (+ (* (Math|Vector|RotateVector (Math|Vector|Normalize (- (Transformation|GetSocketLocation (Variables|/Script/Engine.Character|GetMesh _asshooter_character) "FloatingHUDSocketRagdoll") _returnvalue)) (Math|Rotator|MakeRotator 0.0 (Math|Random|RandomFloatinRange -1.45 1.45) (Math|Random|RandomFloatinRange -1.45 1.45))) 15.0) _returnvalue) (+ (* (Math|Vector|RotateVector (Math|Vector|Normalize (- (Transformation|GetSocketLocation (Variables|/Script/Engine.Character|GetMesh _asshooter_character) "FloatingHUDSocketRagdoll") _returnvalue)) (Math|Rotator|MakeRotator 0.0 (Math|Random|RandomFloatinRange -1.45 1.45) (Math|Random|RandomFloatinRange -1.45 1.45))) (.WeaponRange (Utilities|Struct|BreakInstantWeaponData (Variables|/Script/ShooterGame.ShooterWeapon|GetInstantConfig _asshooter_weapon_instant)))) _returnvalue)))))
                (:then_1
                  (CallFunction|PlayHitShieldEffect false)
                  (LocalVariables|SetDamageOut 0.0)
                  (CallFunction|TrytoDecreaseElement 1)
                  (Class|PrimalItem|AddItemDurability (Variables|Default|GetDurabilityCostPerReflection)))))))))
    (:then_1
      (return (LocalVariables|GetDamageOut)))))

(fn ClientUpdatedWeaponClipAmmo
  (CallFunction|RefreshAmmoMaterial))

(fn RefreshAmmoMaterial
  (bind _ownerinventory (Variables|Default|GetOwnerInventory))
  (Utilities|IsValid _ownerinventory
    (:Is%20Valid
      (if (not (Networking|IsDedicatedServer _ownerinventory))
        (bind _returnvalue (Class|PrimalItem|GetWeaponClipAmmo))
        (Utilities|FlowControl|Sequence
          (:then_0
            (bind _returnvalue_2 (Class|PrimalItem|GetAttachedComponent 0 0))
            (bind _asmesh_component (Utilities|Casting|CastToMeshComponent _returnvalue_2))
            (bind _asmaterial_instance_dynamic (Utilities|Casting|CastToMaterialInstanceDynamic (Rendering|Material|GetMaterial _asmesh_component 0)))
            (Rendering|Material|SetVectorParameterValue _asmaterial_instance_dynamic "Emissive - Color and Intensity" (Utilities|Struct|MakeLinearColor 1.0 1.0 1.0 (Math|Float|SelectFloat 15.0 0.0 (> _returnvalue 0))) :!class /Script/Engine.MaterialInstanceDynamic))
          (:then_1
            (bind _returnvalue_3 (Class|PrimalItem|GetAttachedComponent 1 0))
            (bind _asmesh_component_2 (Utilities|Casting|CastToMeshComponent _returnvalue_3))
            (bind _asmaterial_instance_dynamic_2 (Utilities|Casting|CastToMaterialInstanceDynamic (Rendering|Material|GetMaterial _asmesh_component_2 0)))
            (Rendering|Material|SetVectorParameterValue _asmaterial_instance_dynamic_2 "Emissive - Color and Intensity" (Utilities|Struct|MakeLinearColor 1.0 1.0 1.0 (Math|Float|SelectFloat 15.0 0.0 (> _returnvalue 0))) :!class /Script/Engine.MaterialInstanceDynamic)))))))

(fn BPAddedAttachments
  (CallFunction|RefreshAmmoMaterial))

(fn BPConsumeProjectileImpact
  (params (theProjectile :type Shooter%20Projectile%20Object%20Reference) (HitResult :type Hit%20Result%20Structure%20%28by%20ref%29))
  (bind _returnvalue (Networking|IsServer theProjectile))
  (bind _lastvelocity (Variables|/Script/ShooterGame.ShooterProjectile|GetLastVelocity theProjectile))
  (bind _damagecauser (Variables|/Script/ShooterGame.ShooterProjectile|GetDamageCauser theProjectile))
  (bind _breplicates (Variables|/Script/Engine.Actor|GetbReplicates theProjectile))
  (bind _ownerinventory (Variables|Default|GetOwnerInventory))
  (bind _instigator (Variables|/Script/Engine.Actor|GetInstigator theProjectile))
  (bind _returnvalue_2 (Components|GetOwner _ownerinventory))
  (Utilities|FlowControl|Sequence
    (:then_0
      (if (not (Variables|/Script/ShooterGame.ShooterProjectile|GetbPreventReflecting theProjectile))
        (Utilities|IsValid _ownerinventory
          (:Is%20Valid
            (bind _asshooter_character (Utilities|Casting|CastToShooterCharacter _returnvalue_2))
            (bind _returnvalue_3 (Class|PrimalCharacter|IsBlockedbyShield _asshooter_character HitResult (Math|Vector|Normalize (- (Transformation|GetActorLocation _asshooter_character) (Transformation|GetActorLocation theProjectile))) false))
            (if _returnvalue_3
              (bind _candecrease (CallFunction|CanElementDecrease 1 false))
              (if _candecrease
                (LocalVariables|SetbConsume true)
                (CallFunction|PlayHitShieldEffect false)
                (if (or (not _breplicates) _returnvalue)
                  (if _returnvalue
                    (CallFunction|TrytoDecreaseElement 1)
                    (Utilities|FlowControl|Sequence
                      (:then_0
                        (Utilities|FlowControl|Sequence :!label _label
                          (:then_0
                            (Utilities|FlowControl|Sequence
                              (:then_0
                                (Utilities|IsValid _damagecauser
                                  (:Is%20Valid
                                    (LocalVariables|SetNewTarget _damagecauser))
                                  (:Is%20Not%20Valid
                                    (Utilities|IsValid _instigator
                                      (:Is%20Valid
                                        (LocalVariables|SetNewTarget _instigator))))))
                              (:then_1
                                (Utilities|IsValid (LocalVariables|GetNewTarget)
                                  (:Is%20Valid
                                    (LocalVariables|SetNewVelocity (* (Math|Vector|Normalize (- (Transformation|GetActorLocation (LocalVariables|GetNewTarget)) (Transformation|GetActorLocation theProjectile))) (Math|Vector|VectorLength _lastvelocity))))
                                  (:Is%20Not%20Valid
                                    (LocalVariables|SetNewVelocity (* _lastvelocity -1.0)))))))
                          (:then_1
                            (Class|ShooterProjectile|NetResetTransformandVelocity theProjectile (+ (Transformation|GetActorLocation theProjectile) (* (Math|Vector|Normalize (LocalVariables|GetNewVelocity)) 4.0)) (Math|Conversions|RotationFromXVector (LocalVariables|GetNewVelocity)) (LocalVariables|GetNewVelocity) (Utilities|Array|MakeArray _returnvalue_2))
                            (if _returnvalue
                              (Class|PrimalCharacter|NetForceUpdateAimedCharacters _asshooter_character (+ (Transformation|GetActorLocation theProjectile) (* (Math|Vector|Normalize (LocalVariables|GetNewVelocity)) 4.0)) (+ (+ (Transformation|GetActorLocation theProjectile) (* (Math|Vector|Normalize (LocalVariables|GetNewVelocity)) 4.0)) (* (Math|Rotator|GetRotationXVector (Math|Conversions|RotationFromXVector (LocalVariables|GetNewVelocity))) 2.4e+04)) 0 false 2e+03)
                              (if _breplicates
                                _)))))
                      (:then_1
                        (Class|PrimalItem|AddItemDurability (Variables|Default|GetDurabilityCostPerReflection))))
                    (else
                      (goto _label))))))))))
    (:then_1
      (return (LocalVariables|GetbConsume)))))

(fn PlayHitShieldEffect
  (params (bLocalOnly :type Boolean))
  (bind _ownerinventory (Variables|Default|GetOwnerInventory))
  (bind _returnvalue (Components|GetOwner _ownerinventory))
  (Utilities|IsValid _ownerinventory
    (:Is%20Valid
      (Utilities|FlowControl|Sequence
        (:then_0
          (if (Networking|IsServer _ownerinventory)
            (if (not bLocalOnly)
              (Class|PrimalItem|ServerSendItemExecCommandtoEveryone "ShieldHit" (Utilities|Struct|MakeBPNetExecParams) false false false))))
        (:then_1
          (if (not (Networking|IsDedicatedServer _ownerinventory))
            (bind _asshooter_character (Utilities|Casting|CastToShooterCharacter _returnvalue))
            (Class|VictoryCore|SpawnActorinWorld (Class|Actor|GetWorld _returnvalue) "/Game/PrimalEarth/General/TekArmorShieldImpactEmitter.TekArmorShieldImpactEmitter_C" "0, 0, 0" "0, 0, 0" (select (Class|PrimalCharacter|IsFirstPerson _asshooter_character) (Variables|/Script/ShooterGame.ShooterCharacter|GetMesh1P _asshooter_character) (Variables|/Script/Engine.Character|GetMesh _asshooter_character)) 0 "RiotShieldAttach" 0 0)))))))

(fn BPClientHandleItemNetExecCommand
  (params (CommandName :type Name :default "None") (ExecParams :type BP%20Net%20Exec%20Params%20Structure%20%28by%20ref%29) (ForPC :type Shooter%20Player%20Controller%20Object%20Reference))
  (Utilities|FlowControl|Sequence
    (:then_0
      (switch name CommandName
        (:ShieldHit
          (CallFunction|PlayHitShieldEffect true))))
    (:then_1
      (return))))

(fn BPInitItemColors
  (return (Variables|/Game/Mods/ArenaMod/ShooterGameState_ArenaMod.ShooterGameState_ArenaMod_C|GetNextColorIds (.AsShooter%20Game%20State%20Arena%20Mod (Utilities|Casting|CastToShooterGameState_ArenaMod (Game|GetGameState (Class|VictoryCore|GetPrimaryWorld)))))))