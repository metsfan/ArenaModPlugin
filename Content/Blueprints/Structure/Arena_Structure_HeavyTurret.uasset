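; Arena-mod heavy turret structure that keeps itself stocked with arena turret bullets.
; On the server it sets AI and range settings, grants ammo after an initial delay, then refills on a looping timer except during overtime; clients apply the heavy turret mesh.
; When turret limits are enabled, placement counts nearby flagged structures plus, server-side, defense-plant crop plots, sends a HUD count and blocks building at the limit.
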(event Custom|DoGiveBullets
  (bind _returnvalue (Default|GetSingletonGameManager (.AsTest%20Game%20Mode%20Arena%20Mod (Utilities|Casting|CastToTestGameMode_ArenaMod (Game|GetGameMode))) "NewEnumerator4"))
  (Utilities|IsValid _returnvalue
    (:Is%20Valid
      (if (not (Variables|/ArenaMod/GameManager/GameManager.GameManager_C|GetIsOvertime _returnvalue))
        (Class|PrimalItem|AddNewItem "/ArenaMod/Blueprints/Weapon/Ammo/Arena_TurretBullet.Arena_TurretBullet_C" (Variables|Default|GetMyInventoryComponent) false false 0.0 false 100 false 0.0 false 0 0.0 false false false)))))

(event Custom|GiveBullets
  (CallFunction|DoGiveBullets))

(event EventBeginPlay
  (|CallParentFunction)
  (if (Networking|IsServer)
    (Utilities|FlowControl|Sequence
      (:then_0
        (Variables|Default|SetAISetting 2 false)
        (Variables|Default|SetRangeSetting 2 false))
      (:then_1
        (Utilities|Time|SetTimerbyEvent (delegate Custom|GiveBullets) 3e+02 true)
        (Utilities|FlowControl|Delay 0 6e+01)
        (Class|PrimalItem|AddNewItem "/ArenaMod/Blueprints/Weapon/Ammo/Arena_TurretBullet.Arena_TurretBullet_C" (Variables|Default|GetMyInventoryComponent) false false 0.0 false 100 false 0.0 false 0 0.0 false false false)))
    (else
      (Utilities|FlowControl|Sequence
        (:then_0
          (Components|SkinnedMesh|SetSkinnedAssetandUpdate (Variables|Default|GetSkeletalMesh1) "/Game/PrimalEarth/WeaponTurret/HeavyTurret/Heavy_Turret_Rig.Heavy_Turret_Rig" true))))))

(fn ConstructionScript
  (|CallParentFunction))

(fn BPIsAllowedtoBuildEx
  (params (OutPlacementData :type Placement%20Data%20Structure%20%28by%20ref%29) (CurrentAllowedReason :type Integer) (PC :type Player%20Controller%20Object%20Reference) (bFinalPlacement :type Boolean) (bChoosingRotation :type Boolean))
  (bind _adjustedlocation (Utilities|Struct|BreakPlacementData OutPlacementData))
  (bind _returnvalue (Class|Actor|GetWorld))
  (LocalVariables|SetbRetVal true)
  (bind _asshooter_game_state (Utilities|Casting|CastToShooterGameState (Game|GetGameState)))
  (bind _asprimal_world_settings (Utilities|Casting|CastToPrimalWorldSettings (Class|World|GetWorldSettings _returnvalue false true)))
  (if (Variables|/Script/ShooterGame.ShooterGameState|GetbLimitTurretsInRange _asshooter_game_state)
    (Utilities|FlowControl|Sequence
      (:then_0
        (Utilities|FlowControl|Sequence
          (:then_0
            (if true
              (bind _returnvalue_2 (Class|PrimalStructure|GetNumStructuresinRangeStructureTypeFlag _returnvalue _adjustedlocation 262144 (Utilities|Array|MakeArray) (Variables|/Script/ShooterGame.ShooterGameState|GetLimitTurretsRange _asshooter_game_state) false false 0 false 0))
              (LocalVariables|SetNumTurrets _returnvalue_2)
              (if (Networking|IsServer)
                (bind _structuresout (Class|PrimalStructure|GetStructuresinRange _returnvalue _adjustedlocation (Variables|/Script/ShooterGame.ShooterGameState|GetLimitTurretsRange _asshooter_game_state) "/Game/PrimalEarth/Structures/BuildingBases/CropPlotBaseBP.CropPlotBaseBP_C" false 0))
                (for _array_element _structuresout
                  (bind _asprimal_structure_item_container_crop_plot (Utilities|Casting|CastToPrimalStructureItemContainer_CropPlot _array_element))
                  (Utilities|Casting|CastToPrimalStructureTurret (Variables|/Script/ShooterGame.PrimalStructureItemContainer_CropPlot|GetMyCropStructure _asprimal_structure_item_container_crop_plot)
                    (:CastFailed
                      (bind _returnvalue_3 (Class|PrimalInventoryComponent|GetItemTemplateQuantity (Variables|/Script/ShooterGame.PrimalStructureItemContainer|GetMyInventoryComponent _asprimal_structure_item_container_crop_plot) "/Game/PrimalEarth/CoreBlueprints/Items/Consumables/Seeds/PrimalItemConsumable_Seed_DefensePlant.PrimalItemConsumable_Seed_DefensePlant_C" 0 true false false false))
                      (if (or (> _returnvalue_3 0) (Utilities|ClassIsChildOf (Variables|/Script/ShooterGame.PrimalStructureItemContainer_CropPlot|GetPlantedCrop _asprimal_structure_item_container_crop_plot) "/Game/PrimalEarth/CoreBlueprints/Items/Consumables/Seeds/PrimalItemConsumable_Seed_DefensePlant.PrimalItemConsumable_Seed_DefensePlant_C"))
                        (LocalVariables|SetNumTurrets (+ (LocalVariables|GetNumTurrets) 1)))))))
              (else
                (bind _structuresout_2 (Class|PrimalStructure|GetStructuresinRange _returnvalue _adjustedlocation (Variables|/Script/ShooterGame.ShooterGameState|GetLimitTurretsRange _asshooter_game_state) "/Game/PrimalEarth/Structures/BuildingBases/StructureTurretBaseBP_Heavy.StructureTurretBaseBP_Heavy_C" false 0))
                (LocalVariables|SetNumTurrets (Utilities|Array|Length _structuresout_2)))))
          (:then_1
            (if (>= (LocalVariables|GetNumTurrets) (Variables|/Script/ShooterGame.ShooterGameState|GetLimitTurretsNum _asshooter_game_state))
              (LocalVariables|SetbRetVal false)))))
      (:then_1
        (if (Pawn|IsLocalPlayerController PC)
          _
          (else
            _))
        (bind _asshooter_player_controller (Utilities|Casting|CastToShooterPlayerController PC))
        (Class|ShooterPlayerController|ClientHUDNotificationTypeParams _asshooter_player_controller (Math|Integer|SelectInt 1010836 1010835 (LocalVariables|GetbRetVal)) (LocalVariables|GetNumTurrets) (Variables|/Script/ShooterGame.ShooterGameState|GetLimitTurretsNum _asshooter_game_state) (Class|VictoryCore|ClassReftoObjectRef (Utilities|GetClass self))))
      (:then_2
        (return (Math|Integer|SelectInt CurrentAllowedReason -15 (LocalVariables|GetbRetVal)))))
    (else
      (return (Math|Integer|SelectInt CurrentAllowedReason -15 (LocalVariables|GetbRetVal))))))