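; Base turret structure Blueprint that enforces the game's limit on how many turrets can stand within range of each other.
; Placement checks count nearby turret-flagged structures, plus server-side crop plots holding defense plant seeds or crops, then notify the player and refuse excess builds.
; On save load, the optional hard limit repeats that count and marks excess turrets inactive, blocking activation and excluding them from counts.
; The HUD shows same-team players the count and warnings.
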(fn ConstructionScript)

(fn BlueprintDrawHUD
  (params (HUD :type Shooter%20HUD%20Object%20Reference) (CenterX :type Float%20%28single-precision%29) (CenterY :type Float%20%28single-precision%29))
  (bind _color (Math|Color|MakeColor 0 0 255 255))
  (bind _canvas (Variables|/Script/Engine.HUD|GetCanvas HUD))
  (bind _normalfont (Variables|/Script/ShooterGame.ShooterHUD|GetNormalFont HUD))
  (bind _canvas_2 (Variables|/Script/Engine.HUD|GetCanvas HUD))
  (if (Variables|Default|GetbTooManyInRangeInactive)
    (Class|Canvas|SetDrawColor _canvas (Math|Color|MakeColor 0 0 255 255))
    (Class|Canvas|BPDrawTextCentered _canvas (Variables|/Script/ShooterGame.ShooterHUD|GetNormalFont HUD) "INACTIVE DUE TO TOO MANY TURRETS IN RANGE! RE-PLACE THIS TURRET!" CenterX (- CenterY 1.2e+02) 1.0 1.0 true true))
  (bind _asshooter_game_state (Utilities|Casting|CastToShooterGameState (Game|GetGameState)))
  (if (Variables|/Script/ShooterGame.ShooterGameState|GetbLimitTurretsInRange _asshooter_game_state)
    (if (== (Variables|/Script/Engine.Actor|GetTargetingTeam (Class|ShooterHUD|GetShooterPC HUD)) (Variables|Default|GetTargetingTeam))
      (bind _returnvalue (Class|PrimalStructure|GetNumStructuresinRangeStructureTypeFlag (Class|Actor|GetWorld) (Transformation|GetActorLocation) 262144 (Utilities|Array|MakeArray) (Variables|/Script/ShooterGame.ShooterGameState|GetLimitTurretsRange _asshooter_game_state) false false 0 false 0))
      (if (> _returnvalue (Variables|/Script/ShooterGame.ShooterGameState|GetLimitTurretsNum _asshooter_game_state))
        (Class|Canvas|SetDrawColor _canvas_2 _color)
        (else
          (Class|Canvas|SetDrawColor _canvas_2 (Math|Color|MakeColor 0 255 0 255))))
      (Class|Canvas|BPDrawTextCentered _canvas_2 _normalfont (Utilities|String|ToString(Text) (Utilities|Text|FormatText "Turrets In Range {0} / {1}" (Utilities|Text|ToText(Integer) _returnvalue) (Utilities|Text|ToText(Integer) (Variables|/Script/ShooterGame.ShooterGameState|GetLimitTurretsNum _asshooter_game_state)))) CenterX (- CenterY 8e+01) 1.0 1.0 true true)
      (if (> _returnvalue (Variables|/Script/ShooterGame.ShooterGameState|GetLimitTurretsNum _asshooter_game_state))
        (Class|Canvas|SetDrawColor _canvas_2 _color)
        (Class|Canvas|BPDrawTextCentered _canvas_2 _normalfont "Too many Turrets in range! Move Turrets to retain functionality!" CenterX (- CenterY 1e+02) 1.0 1.0 true true)))))

(fn BPIsAllowedtoBuildEx
  (params (OutPlacementData :type Placement%20Data%20Structure%20%28by%20ref%29) (CurrentAllowedReason :type Integer) (PC :type Player%20Controller%20Object%20Reference) (bFinalPlacement :type Boolean) (bChoosingRotation :type Boolean))
  (bind _adjustedlocation (Utilities|Struct|BreakPlacementData OutPlacementData))
  (bind _returnvalue (Class|Actor|GetWorld))
  (LocalVariables|SetbRetVal true)
  (bind _asshooter_game_state (Utilities|Casting|CastToShooterGameState (Game|GetGameState)))
  (bind _asprimal_world_settings (Utilities|Casting|CastToPrimalWorldSettings (Class|World|GetWorldSettings (Class|PrimalActor|GetWorld) false true)))
  (if (and (Variables|/Script/ShooterGame.ShooterGameState|GetbLimitTurretsInRange _asshooter_game_state) true)
    (Utilities|FlowControl|Sequence
      (:then_0
        (Utilities|FlowControl|Sequence
          (:then_0
            (bind _returnvalue_2 (Class|PrimalStructure|GetNumStructuresinRangeStructureTypeFlag _returnvalue _adjustedlocation 262144 (Utilities|Array|MakeArray) (Variables|/Script/ShooterGame.ShooterGameState|GetLimitTurretsRange _asshooter_game_state) false false 0 false 0))
            (LocalVariables|SetNumTurrets _returnvalue_2)
            (if (Networking|IsServer)
              (bind _structuresout (Class|PrimalStructure|GetStructuresinRange _returnvalue _adjustedlocation (Variables|/Script/ShooterGame.ShooterGameState|GetLimitTurretsRange _asshooter_game_state) "/Game/PrimalEarth/Structures/BuildingBases/CropPlotBaseBP.CropPlotBaseBP_C" false 0))
              (for _array_element _structuresout
                (bind _asprimal_structure_item_container_crop_plot (Utilities|Casting|CastToPrimalStructureItemContainer_CropPlot _array_element))
                (Utilities|Casting|CastToPrimalStructureTurret (Variables|/Script/ShooterGame.PrimalStructureItemContainer_CropPlot|GetMyCropStructure _asprimal_structure_item_container_crop_plot)
                  (:CastFailed
                    (bind _returnvalue_3 (Class|PrimalInventoryComponent|GetItemTemplateQuantity (Variables|/Script/ShooterGame.PrimalStructureItemContainer|GetMyInventoryComponent _asprimal_structure_item_container_crop_plot) "/Game/PrimalEarth/CoreBlueprints/Items/Consumables/Seeds/PrimalItemConsumable_Seed_DefensePlant.PrimalItemConsumable_Seed_DefensePlant_C" 0 true false false false))
                    (if (or (> _returnvalue_3 0) (Utilities|ClassIsChildOf (Variables|/Script/ShooterGame.PrimalStructureItemContainer_CropPlot|GetPlantedCrop _asprimal_structure_item_container_crop_plot) "/Game/PrimalEarth/CoreBlueprints/Items/Consumables/Seeds/PrimalItemConsumable_Seed_DefensePlant.PrimalItemConsumable_Seed_DefensePlant_C"))
                      (LocalVariables|SetNumTurrets (+ (LocalVariables|GetNumTurrets) 1))))))))
          (:then_1
            (if (>= (LocalVariables|GetNumTurrets) (Variables|/Script/ShooterGame.ShooterGameState|GetLimitTurretsNum _asshooter_game_state))
              (LocalVariables|SetbRetVal false)))))
      (:then_1
        (if (Pawn|IsLocalPlayerController PC)
          _
          (else
            _))
        (bind _asshooter_player_controller (Utilities|Casting|CastToShooterPlayerController PC))
        (Class|ShooterPlayerController|ClientHUDNotificationTypeParams _asshooter_player_controller (Math|Integer|SelectInt 1010836 1010835 (LocalVariables|GetbRetVal)) (LocalVariables|GetNumTurrets) (Variables|/Script/ShooterGame.ShooterGameState|GetLimitTurretsNum _asshooter_game_state) (Class|VictoryCore|ClassReftoObjectRef (Utilities|GetClass self))))
      (:then_2
        (return (Math|Integer|SelectInt CurrentAllowedReason -15 (LocalVariables|GetbRetVal)))))
    (else
      (return (Math|Integer|SelectInt CurrentAllowedReason -15 (LocalVariables|GetbRetVal))))))

(fn BPCanbeActivated
  (return (not (Variables|Default|GetbTooManyInRangeInactive))))

(fn BPUseCountStructureinRange
  (return (not (Variables|Default|GetbTooManyInRangeInactive))))

(fn TurretCheckHardLimit
  (bind _returnvalue (Class|Actor|GetWorld))
  (bind _returnvalue_2 (Transformation|GetActorLocation))
  (bind _self self)
  (bind _asshooter_game_mode (Utilities|Casting|CastToShooterGameMode (Game|GetGameMode)))
  (if (Variables|/Script/ShooterGame.ShooterGameMode|GetbHardLimitTurretsInRange _asshooter_game_mode)
    (Utilities|FlowControl|Sequence
      (:then_0
        (bind _returnvalue_3 (Class|PrimalStructure|GetNumStructuresinRangeStructureTypeFlag _returnvalue _returnvalue_2 262144 (Utilities|Array|MakeArray) (Variables|/Script/ShooterGame.ShooterGameMode|GetLimitTurretsRange _asshooter_game_mode) true true _self false 0))
        (LocalVariables|SetNumTurrets _returnvalue_3)
        (if (Networking|IsServer)
          (bind _structuresout (Class|PrimalStructure|GetStructuresinRange _returnvalue _returnvalue_2 (Variables|/Script/ShooterGame.ShooterGameMode|GetLimitTurretsRange _asshooter_game_mode) "/Game/PrimalEarth/Structures/BuildingBases/CropPlotBaseBP.CropPlotBaseBP_C" true _self))
          (for _array_element _structuresout
            (bind _asprimal_structure_item_container_crop_plot (Utilities|Casting|CastToPrimalStructureItemContainer_CropPlot _array_element))
            (Utilities|Casting|CastToPrimalStructureTurret (Variables|/Script/ShooterGame.PrimalStructureItemContainer_CropPlot|GetMyCropStructure _asprimal_structure_item_container_crop_plot)
              (:CastFailed
                (bind _returnvalue_4 (Class|PrimalInventoryComponent|GetItemTemplateQuantity (Variables|/Script/ShooterGame.PrimalStructureItemContainer|GetMyInventoryComponent _asprimal_structure_item_container_crop_plot) "/Game/PrimalEarth/CoreBlueprints/Items/Consumables/Seeds/PrimalItemConsumable_Seed_DefensePlant.PrimalItemConsumable_Seed_DefensePlant_C" 0 true false false false))
                (if (or (> _returnvalue_4 0) (Utilities|ClassIsChildOf (Variables|/Script/ShooterGame.PrimalStructureItemContainer_CropPlot|GetPlantedCrop _asprimal_structure_item_container_crop_plot) "/Game/PrimalEarth/CoreBlueprints/Items/Consumables/Seeds/PrimalItemConsumable_Seed_DefensePlant.PrimalItemConsumable_Seed_DefensePlant_C"))
                  (LocalVariables|SetNumTurrets (+ (LocalVariables|GetNumTurrets) 1))))))))
      (:then_1
        (if (>= (LocalVariables|GetNumTurrets) (Variables|/Script/ShooterGame.ShooterGameMode|GetLimitTurretsNum _asshooter_game_mode))
          (Variables|Default|SetbTooManyInRangeInactive true false)
          (if (Variables|Default|GetbContainerActivated)
            (Class|PrimalStructure|SetContainerActive false))
          (else
            (Variables|Default|SetbTooManyInRangeInactive false false)))))))

(fn BPPostLoadedfromSaveGame
  (CallFunction|TurretCheckHardLimit))