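; Base auto turret for the Arena mod that feeds itself ammo, pays out currency and ignores teammates.
; A server Tick timer moves ammo from a finite reserve into inventory, pausing in overtime unless player-crafted; the turret demolishes when both empty.
; Teammates can buy refills from that reserve on crafted turrets with Hexagons.
; Crafted-turret kills reward the builder, and lethal damage rewards the destroying player, resolved from C4 or pawn damage causers.
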(event EventTick
  (params (DeltaSeconds :type Float%20%28single-precision%29))
  (bind _givebulletsinterval (Variables|Default|GetGiveBulletsInterval))
  (|CallParentFunction DeltaSeconds)
  (if (Networking|IsServer)
    (Utilities|FlowControl|Sequence
      (:then_0
        (Variables|Internal|SetTimeElapsed (+ DeltaSeconds (Variables|Internal|GetTimeElapsed))))
      (:then_1
        (if (>= (Variables|Internal|GetTimeElapsed) _givebulletsinterval)
          (Utilities|FlowControl|Sequence
            (:then_0
              (CallFunction|GiveBullets (Math|Integer|SelectInt (Variables|Default|GetInitialAmmoAmount) (Variables|Default|GetMaxAmmoAddition) (Variables|Internal|GetFirst)) (Variables|Internal|GetFirst)))
            (:then_1
              (Variables|Internal|SetTimeElapsed (- (Variables|Internal|GetTimeElapsed) _givebulletsinterval)))
            (:then_2
              (Variables|Internal|SetFirst false))))))))

(event EventBeginPlay
  (|CallParentFunction)
  (if (Networking|IsServer)
    (Utilities|FlowControl|Sequence
      (:then_0
        (Variables|Default|SetAISetting 2 false)
        (Variables|Default|SetRangeSetting 2 false))
      (:then_1
        (Variables|Internal|SetTimeElapsed (- (Variables|Default|GetGiveBulletsInterval) (Variables|Default|GetInitialGiveBulletsDelay)))
        (Variables|Internal|SetFirst true)))))

(fn ConstructionScript)

(fn GiveBullets
  (params (MaxAmount :type Integer) (Initial :type Boolean))
  (bind _ammoitemtemplate (Variables|Default|GetAmmoItemTemplate))
  (bind _myinventorycomponent (Variables|Default|GetMyInventoryComponent))
  (bind _returnvalue (Default|GetSingletonGameManager (.AsTest%20Game%20Mode%20Arena%20Mod (Utilities|Casting|CastToTestGameMode_ArenaMod (Game|GetGameMode))) "NewEnumerator4"))
  (Utilities|IsValid _returnvalue
    (:Is%20Valid
      (if (and (or (not (Variables|/ArenaMod/GameManager/GameManager.GameManager_C|GetIsOvertime _returnvalue)) (Variables|Default|GetPlayerCrafted)) (> (Variables|Default|GetReserveAmmo) 0))
        (Utilities|FlowControl|Sequence :!label _label
          (:then_0
            (bind _returnvalue_2 (Class|PrimalInventoryComponent|GetItemTemplateQuantity _myinventorycomponent _ammoitemtemplate 0 true false false false))
            (LocalVariables|SetAmountToAdd (Math|Integer|Clamp(Integer) (- (Variables|Default|GetMaxAmmo) _returnvalue_2) 0 (Math|Integer|Min(Integer) MaxAmount (Variables|Default|GetReserveAmmo)))))
          (:then_2
            (if (> (LocalVariables|GetAmountToAdd) 0)
              (Utilities|FlowControl|Sequence
                (:then_0
                  (Class|PrimalItem|AddNewItem _ammoitemtemplate _myinventorycomponent false false 0.0 false (LocalVariables|GetAmountToAdd) false 0.0 false 0 0.0 false false false))
                (:then_1
                  (if (not Initial)
                    (Variables|Default|SetReserveAmmo (- (Variables|Default|GetReserveAmmo) (LocalVariables|GetAmountToAdd)))))))))))
    (:Is%20Not%20Valid
      (goto _label))))

(fn BPNotifyInventoryItemChange
  (params (bIsItemAdd :type Boolean) (theItem :type Primal%20Item%20Object%20Reference) (bEquipItem :type Boolean))
  (if (and (== (Utilities|Array|Length (Variables|/Script/ShooterGame.PrimalInventoryComponent|GetInventoryItems (Variables|Default|GetMyInventoryComponent))) 0) (== (Variables|Default|GetReserveAmmo) 0))
    (Class|PrimalStructure|Demolish 0 0)))

(fn BPGetMultiUseEntries
  (params (ForPC :type Player%20Controller%20Object%20Reference) (MultiUseEntries :type Array%20of%20Multi%20Use%20Entry%20Structures))
  (Utilities|FlowControl|Sequence
    (:then_0
      (Utilities|Array|Clear MultiUseEntries))
    (:then_1
      (if (Math|Boolean|ANDBoolean (Variables|Default|GetPlayerCrafted) (<= (Variables|Default|GetNumBullets) (- (Variables|Default|GetMaxAmmo) (Variables|Default|GetMaxAmmoAddition))) (== (Variables|/Script/Engine.Actor|GetTargetingTeam ForPC) (Variables|Default|GetTargetingTeam)))
        (Utilities|Array|Add MultiUseEntries (Utilities|Struct|MakeMultiUseEntry 0 "Add Ammo (1000 Hexagons)" 8787 0 false (< (Variables|/ArenaMod/PlayerControllerBlueprint_ArenaMod.PlayerControllerBlueprint_ArenaMod_C|GetGameCurrencyAmount (.AsPlayer%20Controller%20Blueprint%20Arena%20Mod (Utilities|Casting|CastToPlayerControllerBlueprint_ArenaMod ForPC))) (Variables|Default|GetRefillHexagonsCost)) false false false false false false false false false false false false 0 false 0 "(B=175,G=175,R=175,A=255)" "(B=255,G=255,R=255,A=255)" 1.0 1.0))))
    (:then_2
      (return MultiUseEntries))))

(fn BPTryMultiUse
  (params (ForPC :type Player%20Controller%20Object%20Reference) (UseIndex :type Integer))
  (bind _refillhexagonscost (Variables|Default|GetRefillHexagonsCost))
  (Utilities|FlowControl|Sequence
    (:then_0
      (if (Math|Boolean|ANDBoolean (== UseIndex 8787) (Variables|Default|GetPlayerCrafted) (== (Variables|/Script/Engine.Actor|GetTargetingTeam ForPC) (Variables|Default|GetTargetingTeam)))
        (bind _asplayer_controller_blueprint_arena_mod (Utilities|Casting|CastToPlayerControllerBlueprint_ArenaMod ForPC))
        (if (>= (Variables|/ArenaMod/PlayerControllerBlueprint_ArenaMod.PlayerControllerBlueprint_ArenaMod_C|GetGameCurrencyAmount _asplayer_controller_blueprint_arena_mod) _refillhexagonscost)
          (Default|RemoveGameCurrency _asplayer_controller_blueprint_arena_mod _refillhexagonscost)
          (CallFunction|GiveBullets (Variables|Default|GetMaxAmmoAddition) false))))
    (:then_1
      (return false))))

(fn OnKilledPlayer
  (params (Character :type Shooter%20Character%20Object%20Reference))
  (Utilities|Casting|CastToPlayerPawnTest_Child_ArenaMod Character)
  (if (Variables|Default|GetPlayerCrafted)
    (Utilities|IsValid (Variables|Default|GetPlayerOwner)
      (:Is%20Valid
        (bind _asplayer_controller_blueprint_arena_mod (Utilities|Casting|CastToPlayerControllerBlueprint_ArenaMod (Variables|Default|GetPlayerOwner)))
        (if (> (Variables|/ArenaMod/PlayerControllerBlueprint_ArenaMod.PlayerControllerBlueprint_ArenaMod_C|GetCurrentGameId _asplayer_controller_blueprint_arena_mod) 0)
          (Default|AddGameCurrency _asplayer_controller_blueprint_arena_mod (Variables|Default|GetPlayerKillHexagonBonus))
          (Default|AddCurrency _asplayer_controller_blueprint_arena_mod (Variables|Default|GetPlayerKillShardBonus))
          (else
            (Variables|Default|SetPlayerOwner 0)))))))

(fn BPSetPlayerConstructor
  (params (PC :type Player%20Controller%20Object%20Reference))
  (Variables|Default|SetPlayerOwner PC))

(fn BPTurretPreventsTargeting
  (params (PotentialTarget :type Primal%20Character%20Object%20Reference))
  (Utilities|FlowControl|Sequence
    (:then_0
      (bind _asprimal_dino_character (Utilities|Casting|CastToPrimalDinoCharacter PotentialTarget))
      (LocalVariables|SetbRetVal (Class|PrimalCharacter|IsWildSlow _asprimal_dino_character)))
    (:then_2
      (return (or (== (Variables|/Script/Engine.Actor|GetTargetingTeam PotentialTarget) (Variables|Default|GetTargetingTeam)) (LocalVariables|GetbRetVal))))))

(fn ReceiveAnyDamage
  (params (Damage :type Float%20%28single-precision%29) (DamageType :type Damage%20Type%20Object%20Reference) (InstigatedBy :type Controller%20Object%20Reference) (DamageCauser :type Actor%20Object%20Reference))
  (if (Math|Boolean|ANDBoolean (<= (- (Variables|Default|GetHealth) Damage) 0.0) (not (Variables|Default|GetDestroyingCurrencyGiven)) (Networking|IsServer))
    (Utilities|FlowControl|Sequence
      (:then_0
        (bind _asarena_c4charge_structure (Utilities|Casting|CastToArena_C4ChargeStructure DamageCauser))
        (bind _pc (Default|GetPCforPlayerId (.AsTest%20Game%20Mode%20Arena%20Mod (Utilities|Casting|CastToTestGameMode_ArenaMod (Game|GetGameMode))) (Variables|/ArenaMod/Blueprints/Weapon/Ammo/Arena_C4ChargeStructure.Arena_C4ChargeStructure_C|GetOwnerLinkedPlayerID _asarena_c4charge_structure)))
        (LocalVariables|SetDestroyingPlayer _pc))
      (:then_1
        (bind _asplayer_pawn_test_child_arena_mod (Utilities|Casting|CastToPlayerPawnTest_Child_ArenaMod DamageCauser))
        (bind _returnvalue (Class|Actor|GetOwnerController _asplayer_pawn_test_child_arena_mod))
        (bind _asplayer_controller_blueprint_arena_mod (Utilities|Casting|CastToPlayerControllerBlueprint_ArenaMod _returnvalue))
        (LocalVariables|SetDestroyingPlayer _asplayer_controller_blueprint_arena_mod))
      (:then_2
        (Utilities|IsValid (LocalVariables|GetDestroyingPlayer)
          (:Is%20Valid
            (Default|AddGameCurrency (LocalVariables|GetDestroyingPlayer) (Variables|Default|GetGameCurrencyDestructionReward))
            (Variables|Default|SetDestroyingCurrencyGiven true)))))))