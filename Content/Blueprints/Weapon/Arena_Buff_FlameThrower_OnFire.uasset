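; Arena flamethrower "on fire" buff that burns the affected character over time.
; On server tick it applies fire damage once per second as a clamped percentage of max health, credited to the buff's damage causer, using a no-buff fire damage type.
; The buff refuses watered characters and deactivates itself if the victim becomes watered.
; Non-dedicated instances attach a flame light particle to the character's mesh and switch it off on deactivation.
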(fn ConstructionScript)

(fn BPCustomAllowAddBuff
  (params (ForCharacter :type Primal%20Character%20Object%20Reference) (DamageCauser :type Actor%20Object%20Reference))
  (return (not (Class|PrimalCharacter|IsWatered ForCharacter))))

(fn ReceiveTick
  (params (DeltaSeconds :type Float%20%28single-precision%29))
  (bind _buffdamagecauser (Variables|Default|GetBuffDamageCauser))
  (Utilities|FlowControl|Sequence
    (:then_0
      (if (and (Networking|IsServer) (not (Variables|Default|GetbDeactivated)))
        (bind _asprimal_character (Utilities|Casting|CastToPrimalCharacter (Variables|Default|GetInstigator)))
        (if (CallFunction|BPCustomAllowAddBuff _asprimal_character)
          (bind _returnvalue (Class|VictoryCore|StaticGetTimeSince (Class|PrimalActor|GetWorld) (Variables|Default|GetLastDamageTime)))
          (if (>= _returnvalue 1.0)
            (Variables|Default|SetLastDamageTime (Utilities|Time|GetGameTimeinSeconds))
            (Game|Damage|ApplyDamage _asprimal_character (Math|Float|Clamp(Float) (* (Class|PrimalCharacter|GetMaxHealth _asprimal_character) (Variables|Default|GetMaxHealthPercentDamagePerSecond)) (Variables|Default|GetMinDamagePerSecond) (Variables|Default|GetMaxDamagePerSecond)) (Class|PrimalActor|GetCharacterController _buffdamagecauser) _buffdamagecauser "/Game/PrimalEarth/CoreBlueprints/DamageTypes/ShooterDamageTypeBP_Fire_NoBuff.ShooterDamageTypeBP_Fire_NoBuff_C"))
          (else
            (Class|PrimalBuff|BPDeactivate)))))
    (:then_1
      (|CallParentFunction DeltaSeconds))))

(fn BPSetupforInstigator
  (params (ForInstigator :type Actor%20Object%20Reference))
  (if (not (Networking|IsDedicatedServer))
    (bind _asprimal_character (Utilities|Casting|CastToPrimalCharacter ForInstigator))
    (bind _returnvalue (AddComponent|AddParticleSystemComponent true (Transformation|GetSocketTransform (Variables|/Script/Engine.Character|GetMesh _asprimal_character) "None" "RTS_World")))
    (Effects|Components|ParticleSystem|SetTemplate _returnvalue "/Game/PrimalEarth/Effects/Particles/Gameplay/EnflamedLight.EnflamedLight")
    (Variables|Default|SetExtraLight _returnvalue)
    (Class|SceneComponent|Attachto _returnvalue (Variables|/Script/Engine.Character|GetMesh _asprimal_character) (Class|SkinnedMeshComponent|GetSocketBoneName (Variables|/Script/Engine.Character|GetMesh _asprimal_character) "buffsocketcenterdynamic") "SnapToTarget" true)))

(fn BPDeactivated
  (params (ForInstigator :type Actor%20Object%20Reference))
  (Components|Activation|Deactivate (Variables|Default|GetExtraLight)))