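; Explosive demolition damage type that removes friendly fire from Arena C4 charge structure blasts.
; BPAdjustDamage zeroes damage when the victim shares the charge's targeting team, except for the shooter character whose linked player ID matches the charge owner.
; Same-team victims that are not shooter characters always take zero.
; Damage from any other causer passes through unchanged.
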(fn BPAdjustDamage
  (params (Victim :type Actor%20Object%20Reference) (IncomingDamage :type Float%20%28single-precision%29) (TheDamageEvent :type Damage%20Event%20Structure) (EventInstigator :type Controller%20Object%20Reference) (DamageCauser :type Actor%20Object%20Reference))
  (bind _targetingteam (Variables|/Script/Engine.Actor|GetTargetingTeam DamageCauser))
  (bind _targetingteam_2 (Variables|/Script/Engine.Actor|GetTargetingTeam Victim))
  (bind _returnvalue (== _targetingteam_2 _targetingteam))
  (LocalVariables|SetOut IncomingDamage)
  (Utilities|FlowControl|Sequence
    (:then_0
      (bind _asarena_c4charge_structure (Utilities|Casting|CastToArena_C4ChargeStructure DamageCauser))
      (bind _asshooter_character (Utilities|Casting|CastToShooterCharacter Victim)
        (:then
          (bind _returnvalue_2 (Class|ShooterCharacter|LinkedPlayerIDString _asshooter_character))
          (if (and _returnvalue (Utilities|Enum|NotEqual(Enum) _returnvalue_2 (Variables|/ArenaMod/Blueprints/Weapon/Ammo/Arena_C4ChargeStructure.Arena_C4ChargeStructure_C|GetOwnerLinkedPlayerID _asarena_c4charge_structure)))
            (LocalVariables|SetOut 0.0)))
        (:CastFailed
          (if _returnvalue
            (LocalVariables|SetOut 0.0)))))
    (:then_1
      (return (LocalVariables|GetOut)))))