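; Arena mod child of the empty cryopod weapon that limits dino capture to the player's own or player-unowned dinos.
; CanCapture adds an owner-ID check to the parent's rules.
; ReportSuccess runs the parent logic, then passes the captured dino to the Arena player controller's CryoPersonalDino.
; ManualIngest directly packs a given dino's identity, stats, saddle and timers into item custom data, drops its inventory and destroys it.
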(event Custom|ManualIngest
  (params (Dino :type Primal%20Dino%20Character%20Object%20Reference))
  (Utilities|FlowControl|Sequence
    (:then_0
      (Variables|Default|SetCapturingDino Dino))
    (:then_1
      (bind _outdinodata (Class|PrimalDinoCharacter|GetDinoData (Variables|Default|GetCapturingDino)))
      (bind _bytes (CallFunction|GetSaddleData))
      (Class|PrimalItem|SetCustomItemData (Variables|Default|GetAssociatedPrimalItem) (Utilities|Struct|MakeCustomItemData "Dino" (Utilities|Array|MakeArray (.DinoNameInMap (Utilities|Struct|BreakARKDinoData _outdinodata)) (.DinoName (Utilities|Struct|BreakARKDinoData _outdinodata))) (CallFunction|GetCharacterStatsasFloats (Variables|Default|GetCapturingDino)) (Utilities|Array|MakeArray) (Utilities|Array|MakeArray (.DinoClass (Utilities|Struct|BreakARKDinoData _outdinodata))) (Utilities|Array|MakeArray) (Utilities|Struct|MakeCustomItemByteArrays (Utilities|Array|MakeArray (Utilities|Struct|MakeCustomItemByteArray (.DinoData (Utilities|Struct|BreakARKDinoData _outdinodata))) (Utilities|Struct|MakeCustomItemByteArray _bytes))) (Utilities|Struct|MakeCustomItemDoubles (Utilities|Array|MakeArray (Utilities|Time|GetGameTimeinSeconds) (- (Variables|/Script/ShooterGame.PrimalDinoCharacter|GetBabyNextCuddleTime (Variables|Default|GetCapturingDino)) (Utilities|Time|GetGameTimeinSeconds)) (Variables|/Script/ShooterGame.PrimalDinoCharacter|GetNextAllowedMatingTime (Variables|Default|GetCapturingDino))))))
      (Class|PrimalItem|UpdatedItem (Variables|Default|GetAssociatedPrimalItem) true)
      (Class|PrimalInventoryComponent|BPDropInventoryDeposit (Variables|/Script/ShooterGame.PrimalCharacter|GetMyInventoryComponent (Variables|Default|GetCapturingDino)) (+ (Class|VictoryCore|TimeSeconds (Class|PrimalActor|GetWorld)) (Math|Conversions|ToFloat(Integer) (Variables|/Script/ShooterGame.PrimalDinoCharacter|GetTamedCorpseLifespan (Variables|Default|GetCapturingDino)))))
      (Actor|DestroyActor (Variables|Default|GetCapturingDino)))))

(event EventReportSuccess
  (|CallParentFunction)
  (Utilities|FlowControl|Sequence
    (:then_0
      (bind _returnvalue (Class|Actor|GetOwnerController (Components|GetOwner (Variables|/Script/ShooterGame.PrimalItem|GetOwnerInventory (Variables|Default|GetAssociatedPrimalItem)))))
      (bind _asplayer_controller_blueprint_arena_mod (Utilities|Casting|CastToPlayerControllerBlueprint_ArenaMod _returnvalue))
      (Default|CryoPersonalDino _asplayer_controller_blueprint_arena_mod (Variables|Default|GetCapturingDino)))))

(fn ConstructionScript
  (|CallParentFunction))

(fn CanCapture
  (params (Dino :type Primal%20Dino%20Character%20Object%20Reference))
  (bind _owningplayerid (Variables|/Script/ShooterGame.PrimalDinoCharacter|GetOwningPlayerID Dino))
  (Utilities|FlowControl|Sequence
    (:then_0
      (bind _returnvalue (Class|Actor|GetOwnerController (Components|GetOwner (Variables|/Script/ShooterGame.PrimalItem|GetOwnerInventory (Variables|Default|GetAssociatedPrimalItem)))))
      (bind _asplayer_controller_blueprint_arena_mod (Utilities|Casting|CastToPlayerControllerBlueprint_ArenaMod _returnvalue))
      (bind _returnvalue_2 (Class|ShooterPlayerController|LinkedPlayerIDString _asplayer_controller_blueprint_arena_mod))
      (LocalVariables|SetOut (and (or (== _owningplayerid 0) (Utilities|Enum|Equal(Enum) _returnvalue_2 (Utilities|String|ToString(Integer) _owningplayerid))) (|CallParentFunction Dino))))
    (:then_1
      (return (LocalVariables|GetOut)))))