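; Arena mod child of the cryopod that restricts which dinos a team can deploy.
; Its CanDeploy override asks TestGameMode_ArenaMod whether the dino is tamable by the owner's team, treating an empty error string as approval.
; Only approved deployments continue to the parent check, which supplies the final result, location and failure reason.
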(fn CanDeploy
  (params (Class :type Primal%20Dino%20Character%20Class%20Reference) (Location :type Vector :default "0, 0, 0") (SpawningActor :type Actor%20Object%20Reference) (IgnoreActor :type Actor%20Object%20Reference))
  (bind _ownerinventory (Variables|Default|GetOwnerInventory))
  (Utilities|FlowControl|Sequence
    (:then_0
      (bind _astest_game_mode_arena_mod (Utilities|Casting|CastToTestGameMode_ArenaMod (Game|GetGameMode _ownerinventory)))
      (bind _error (Default|IsDinoTamablebyTeam _astest_game_mode_arena_mod Class (Variables|/Script/Engine.Actor|GetTargetingTeam (Components|GetOwner _ownerinventory))))
      (LocalVariables|SetError _error)
      (LocalVariables|SetSuccess (== (Utilities|String|Len _error) 0)))
    (:then_1
      (if (LocalVariables|GetSuccess)
        (bind (_can _newlocation _failurereason) (|CallParentFunction Class Location SpawningActor IgnoreActor))
        (LocalVariables|SetSuccess _can)
        (LocalVariables|SetOutLocation _newlocation)
        (LocalVariables|SetError _failurereason)))
    (:then_2
      (return (LocalVariables|GetSuccess) (LocalVariables|GetOutLocation) (LocalVariables|GetError)))))