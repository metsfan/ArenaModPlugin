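; Tek sword melee weapon that grants its item's buff while equipped and spends ammo (element) per swing and per qualifying hit.
; Attacks are blocked during certain Tek punch buff states, and an empty clip triggers a reload.
; Server hit checks respect team and PvE rules, set cost by target type, and boost damage against structures without specific settings.
; Replicated ammo state toggles client glow, particles and audio, with particles tinted by item color.
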(event Custom|PlayAttackSound
  (Audio|SpawnSoundAttached "/Game/PrimalEarth/TekTier/TekArmor/Sounds/TekSword_Swing_Cue.TekSword_Swing_Cue" (Class|ShooterWeapon|GetWeaponMesh) "None" "0, 0, 0" "0, 0, 0" "SnapToTarget" true 1.0 1.0 0.0 0 0))

(event Custom|NetDoPlayMeleeAttackSound
  (if (not (Networking|IsDedicatedServer))
    (if (not (Class|ShooterWeapon|IsLocallyOwned))
      (CallFunction|PlayAttackSound))))

(fn ConstructionScript
  (|CallParentFunction))

(fn BPAppliedPrimalItemtoWeapon
  (bind _associatedprimalitem (Variables|Default|GetAssociatedPrimalItem))
  (bind (_outcolor _returnvalue) (Class|PrimalItem|GetItemCustomColor _associatedprimalitem))
  (bind (_r _g _b) (Utilities|Struct|BreakLinearColor _outcolor))
  (if (not (Networking|IsDedicatedServer))
    (Utilities|IsValid _associatedprimalitem
      (:Is%20Valid
        (if _returnvalue
          (Effects|Components|ParticleSystem|SetVectorParameter (Variables|Default|GetParticleSystem1) "Color0" (Math|Vector|MakeVector _r _g _b)))))))

(fn BPHandleMeleeAttack
  (bind _returnvalue (Class|ShooterWeapon|IsLocallyOwned))
  (bind _currentammoinclip (Variables|Default|GetCurrentAmmoInClip))
  (bind _returnvalue_2 (> _currentammoinclip 0))
  (bind _asbuff_tek_armor_sword (Utilities|Casting|CastToBuff_TekArmor_Sword (Class|PrimalCharacter|GetBuff (Variables|Default|GetMyPawn) "/Game/PrimalEarth/CoreBlueprints/Buffs/Buff_TekArmor_Sword.Buff_TekArmor_Sword_C")))
  (if (not (Math|Boolean|ORBoolean (Utilities|Enum|Equal(Enum) (Variables|/Game/PrimalEarth/CoreBlueprints/Buffs/Buff_TekArmor_Sword.Buff_TekArmor_Sword_C|GetCurrentTekPunchState _asbuff_tek_armor_sword) "NewEnumerator5") (Utilities|Enum|Equal(Enum) (Variables|/Game/PrimalEarth/CoreBlueprints/Buffs/Buff_TekArmor_Sword.Buff_TekArmor_Sword_C|GetCurrentTekPunchState _asbuff_tek_armor_sword) "NewEnumerator6") (Utilities|Enum|Equal(Enum) (Variables|/Game/PrimalEarth/CoreBlueprints/Buffs/Buff_TekArmor_Sword.Buff_TekArmor_Sword_C|GetCurrentTekPunchState _asbuff_tek_armor_sword) "NewEnumerator1") (Utilities|Enum|Equal(Enum) (Variables|/Game/PrimalEarth/CoreBlueprints/Buffs/Buff_TekArmor_Sword.Buff_TekArmor_Sword_C|GetCurrentTekPunchState _asbuff_tek_armor_sword) "NewEnumerator4")))
    (if _returnvalue_2
      (Class|ShooterWeapon|DoMeleeAttack)
      (Utilities|FlowControl|Sequence
        (:then_0
          (if _returnvalue
            (CallFunction|PlayAttackSound)))
        (:then_1
          (if (Networking|IsServer)
            (CallFunction|NetDoPlayMeleeAttackSound)
            (Class|ShooterWeapon|UseAmmo (Variables|Default|GetAmmoCostPerSwing))
            (if (not _returnvalue_2)
              (Class|ShooterWeapon|ServerStartReload)))))
      (elif _returnvalue
        (Class|ShooterWeapon|ServerStartReload)))))

(fn ReceiveTick
  (params (DeltaSeconds :type Float%20%28single-precision%29))
  (bind _particlesystem1 (Variables|Default|GetParticleSystem1))
  (bind _particlesystem2 (Variables|Default|GetParticleSystem2))
  (bind _mypawn (Variables|Default|GetMyPawn))
  (bind _audio1 (Variables|Default|GetAudio1))
  (Utilities|FlowControl|Sequence
    (:then_0
      (if (Networking|IsServer)
        (Variables|Default|SetbRepHasAmmo (> (Variables|Default|GetCurrentAmmoInClip) 0) true)))
    (:then_1
      (if (not (Networking|IsDedicatedServer))
        (LocalVariables|SetbDoActive (Math|Boolean|ANDBoolean (Variables|Default|GetbRepHasAmmo) (Utilities|IsValid _mypawn) (Variables|/Script/ShooterGame.ShooterCharacter|GetbIsConnected _mypawn)))
        (Utilities|FlowControl|Sequence
          (:then_0
            (bind _asmaterial_instance_dynamic (Utilities|Casting|CastToMaterialInstanceDynamic (Rendering|Material|GetMaterial (Variables|Default|GetSM1P) 1)))
            (Rendering|Material|SetScalarParameterValue _asmaterial_instance_dynamic "Opacity" (select (LocalVariables|GetbDoActive) 0.5 0.0) :!class /Script/Engine.MaterialInstanceDynamic))
          (:then_1
            (bind _asmaterial_instance_dynamic_2 (Utilities|Casting|CastToMaterialInstanceDynamic (Rendering|Material|GetMaterial (Variables|Default|GetSM3P) 1)))
            (Rendering|Material|SetScalarParameterValue _asmaterial_instance_dynamic_2 "Opacity" (select (LocalVariables|GetbDoActive) 0.5 0.0) :!class /Script/Engine.MaterialInstanceDynamic))
          (:then_2
            (if (Math|Boolean|Equal(Boolean) (Variables|/Script/Engine.ParticleSystemComponent|GetbWasDeactivated _particlesystem1) (LocalVariables|GetbDoActive))
              (if (LocalVariables|GetbDoActive)
                (Components|Activation|Activate _particlesystem1 false)
                (else
                  (Components|Activation|Deactivate _particlesystem1)))))
          (:then_3
            (if (Math|Boolean|Equal(Boolean) (Variables|/Script/Engine.ParticleSystemComponent|GetbWasDeactivated _particlesystem2) (LocalVariables|GetbDoActive))
              (if (LocalVariables|GetbDoActive)
                (Components|Activation|Activate _particlesystem2 false)
                (else
                  (Components|Activation|Deactivate _particlesystem2)))))
          (:then_4
            (if (Math|Boolean|NotEqual(Boolean) (LocalVariables|GetbDoActive) (Components|Activation|IsActive _audio1))
              (if (LocalVariables|GetbDoActive)
                (Components|Activation|Activate _audio1 false)
                (else
                  (Components|Activation|Deactivate _audio1))))))))))

(fn StartUnequipEvent
  (bind _associatedprimalitem (Variables|Default|GetAssociatedPrimalItem))
  (|CallParentFunction)
  (bind _asshooter_character (Utilities|Casting|CastToShooterCharacter (Components|GetOwner)))
  (Class|PrimalCharacter|DeactivateBuffs _asshooter_character (Utilities|ResolveSoftReference (Variables|/Script/ShooterGame.PrimalItem|GetBuffToGiveOwnerCharacter _associatedprimalitem)) _associatedprimalitem false))

(fn BPStartEquippedNotify
  (bind _associatedprimalitem (Variables|Default|GetAssociatedPrimalItem))
  (bind _asprimal_character (Utilities|Casting|CastToPrimalCharacter (Components|GetOwner)))
  (Class|PrimalBuff|StaticAddBuff (Utilities|ResolveSoftReference (Variables|/Script/ShooterGame.PrimalItem|GetBuffToGiveOwnerCharacter _associatedprimalitem)) _asprimal_character _associatedprimalitem 0 false))

(fn BPWeaponDealDamage
  (params (Impact :type Hit%20Result%20Structure%20%28by%20ref%29) (ShootDir :type Vector%20%28by%20ref%29 :default "0, 0, 0") (DamageAmount :type Integer) (DamageType :type Damage%20Type%20Class%20Reference) (Impulse :type Float%20%28single-precision%29))
  (LocalVariables|SetOutDamage DamageAmount)
  (Utilities|FlowControl|Sequence
    (:then_0
      (bind _bextradamage (CallFunction|AppliedDamagetoTarget (.HitActor (Collision|BreakHitResult Impact)) 1.0))
      (if _bextradamage
        (LocalVariables|SetOutDamage (Math|Float|Floor (* (LocalVariables|GetOutDamage) (Variables|Default|GetExtraStructureDamageMultiplier))))))
    (:then_1
      (return (LocalVariables|GetOutDamage)))))

(fn AppliedDamagetoTarget
  (params (DamageTarget :type Actor%20Object%20Reference) (ElementCostMultiplier :type Float%20%28double-precision%29) (DamageIn :type Integer))
  (bind _targetingteam (Variables|/Script/Engine.Actor|GetTargetingTeam DamageTarget))
  (Utilities|FlowControl|Sequence
    (:then_0
      (if (Networking|IsServer)
        (bind _asshooter_game_state (Utilities|Casting|CastToShooterGameState (Game|GetGameState)))
        (if (and (or (not (Variables|/Script/ShooterGame.ShooterGameState|GetbServerPVE _asshooter_game_state)) (<= _targetingteam 50000)) (!= (Variables|/Script/Engine.Actor|GetTargetingTeam (Variables|Default|GetMyPawn)) _targetingteam))
          (Utilities|FlowControl|Sequence
            (:then_0
              (Utilities|Casting|CastToPrimalCharacter DamageTarget
                (:then
                  (LocalVariables|SetAmmoCost (Variables|Default|GetCharacterElementCostPerHit)))
                (:CastFailed
                  (bind _asprimal_structure (Utilities|Casting|CastToPrimalStructure DamageTarget))
                  (if (>= (Utilities|Array|FindItem (Variables|Default|GetSpecificStructureSettings) (Variables|/Script/ShooterGame.PrimalTargetableActor|GetStructureSettingsClass _asprimal_structure)) 0)
                    (LocalVariables|SetAmmoCost (Utilities|Array|Get(acopy) (Variables|Default|GetSpecificStructureSettingsElementCostPerHit) (Utilities|Array|FindItem (Variables|Default|GetSpecificStructureSettings) (Variables|/Script/ShooterGame.PrimalTargetableActor|GetStructureSettingsClass _asprimal_structure))))
                    (else
                      (LocalVariables|SetAmmoCost (Variables|Default|GetGenericStructureSettingsElementCostPerHit))
                      (LocalVariables|SetbDoExtraDamage true))))))
            (:then_1
              (if (> (Math|Float|Ceil (* ElementCostMultiplier (LocalVariables|GetAmmoCost))) 0)
                (Class|ShooterWeapon|UseAmmo (Math|Float|Ceil (* ElementCostMultiplier (LocalVariables|GetAmmoCost))))))))))
    (:then_1
      (return (LocalVariables|GetbDoExtraDamage)))))