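; Arena mod Plant Species Y trap structure that decays over time and removes itself when its immobilized victim is reported dead or unconscious.
; Unless NoCollision is set, a looping self-damage event starts shortly after spawn, applying passive decay damage at a configurable rate.
; Damage adjustment zeroes everything except specific fire, flamethrower, explosion and passive damage types.
; Placement by an Arena player pawn in PassiveMode demolishes it immediately.
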(event Custom|PeriodicDamage
  (bind _self self)
  (Game|Damage|ApplyDamage _self (Variables|Default|GetAmountOfDecay) 0 _self "/Game/PrimalEarth/CoreBlueprints/DamageTypes/DmgType_Passive.DmgType_Passive_C")
  (Utilities|FlowControl|RetriggerableDelay 0 (Variables|Default|GetDecayRate))
  (CallFunction|PeriodicDamage))

(event EventBeginPlay
  (|CallParentFunction)
  (if (not (Variables|Default|GetbNoCollision))
    (Utilities|FlowControl|Delay 0 5.0)
    (CallFunction|PeriodicDamage)))

(fn ConstructionScript)

(fn BPNotifyImmobilizedCharacterIsDead
  (Class|PrimalStructure|Demolish 0 0))

(fn BPNotifyImmobilizedCharacterIsDeadorinConscious
  (params (IsDead :type Boolean) (IsConscious :type Boolean))
  (Class|PrimalStructure|Demolish 0 0))

(fn BPAdjustDamage
  (params (IncomingDamage :type Float%20%28single-precision%29) (TheDamageEvent :type Damage%20Event%20Structure) (EventInstigator :type Controller%20Object%20Reference) (DamageCauser :type Actor%20Object%20Reference) (bIsPointDamage :type Boolean) (PointHitInfo :type Hit%20Result%20Structure))
  (bind _damagetypeclass (Utilities|Struct|BreakDamageEvent TheDamageEvent))
  (return (select (Math|Boolean|ORBoolean (Utilities|ClassIsChildOf _damagetypeclass "/Game/ScorchedEarth/WeaponFlamethrower/DmgType_FlameThrower.DmgType_FlameThrower_C") (Utilities|ClassIsChildOf _damagetypeclass "/Game/PrimalEarth/CoreBlueprints/DamageTypes/ShooterDamageTypeBP_Fire.ShooterDamageTypeBP_Fire_C") (Utilities|ClassIsChildOf _damagetypeclass "/Game/PrimalEarth/CoreBlueprints/DamageTypes/DmgType_Projectile_Fire.DmgType_Projectile_Fire_C") (Utilities|ClassIsChildOf _damagetypeclass "/Game/PrimalEarth/CoreBlueprints/DamageTypes/DmgType_Explosion.DmgType_Explosion_C") (Utilities|ClassIsChildOf _damagetypeclass "/Game/PrimalEarth/CoreBlueprints/DamageTypes/DmgType_Passive.DmgType_Passive_C") (Utilities|ClassIsChildOf _damagetypeclass "/Game/PrimalEarth/CoreBlueprints/DamageTypes/DmgType_Melee_Torpidity_Low_StoneWeapon_Fire.DmgType_Melee_Torpidity_Low_StoneWeapon_Fire_C")) IncomingDamage 0.0)))

(fn BPPlacedStructure
  (params (ForPC :type Player%20Controller%20Object%20Reference))
  (bind _asplayer_pawn_test_child_arena_mod (Utilities|Casting|CastToPlayerPawnTest_Child_ArenaMod (Pawn|GetControlledPawn ForPC)))
  (if (Variables|/ArenaMod/PlayerPawnTest_Child_ArenaMod.PlayerPawnTest_Child_ArenaMod_C|GetPassiveMode _asplayer_pawn_test_child_arena_mod)
    (Class|PrimalStructure|Demolish 0 0)))