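; Arena variant of the Tek Rifle projectile that limits its effect on structures to a maximum range from where it spawned.
; It records its spawn location on BeginPlay and compares the distance travelled against MaxStructureImpactDistance.
; Beyond that range, exploding on a PrimalStructure destroys the projectile, and the radial damage filter ignores structure victims.
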(event EventBeginPlay
  (Variables|Default|SetStartLocation (Transformation|GetActorLocation)))

(event EventOnExplode
  (params (Result :type Hit%20Result%20Structure%20%28by%20ref%29))
  (Utilities|Casting|CastToPrimalStructure (.HitActor (Collision|BreakHitResult Result)))
  (if (> (Math|Vector|VectorLength (- (Transformation|GetActorLocation) (Variables|Default|GetStartLocation))) (Variables|Default|GetMaxStructureImpactDistance))
    (Actor|DestroyActor)))

(fn ConstructionScript)

(fn BPIgnoreRadialDamageVictim
  (params (Victim :type Actor%20Object%20Reference))
  (return (and (Class|Actor|BPIsA Victim "/Script/ShooterGame.PrimalStructure") (> (Math|Vector|VectorLength (- (Transformation|GetActorLocation) (Variables|Default|GetStartLocation))) (Variables|Default|GetMaxStructureImpactDistance)))))