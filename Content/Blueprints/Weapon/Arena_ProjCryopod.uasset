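; Cryopod projectile for the Arena mod that deploys a stored dino where it explodes.
; On explode, the server resolves the owning cryopod weapon, shooter and item, and checks for stored dino data.
; It calls the item's TryDeploy at the projectile's transform, ignoring itself.
; Success triggers the weapon's deploy feedback scaled by the dino class's default capsule radius; failure shows the player a red reason message and triggers failure feedback.
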(event EventOnExplode
  (params (Result :type Hit%20Result%20Structure%20%28by%20ref%29))
  (if (Networking|IsServer)
    (bind _asweap_empty_cryopod (Utilities|Casting|CastToWeapEmptyCryopod (Components|GetOwner self)))
    (bind _asshooter_character (Utilities|Casting|CastToShooterCharacter (Components|GetOwner (Variables|/Script/ShooterGame.PrimalItem|GetOwnerInventory (Variables|/Script/ShooterGame.ShooterWeapon|GetAssociatedPrimalItem _asweap_empty_cryopod)))))
    (bind _returnvalue (Class|Actor|GetOwnerController _asshooter_character))
    (bind _asshooter_player_controller (Utilities|Casting|CastToShooterPlayerController _returnvalue))
    (bind _asarena_primal_item_weapon_empty_cryopod_copy (Utilities|Casting|CastToArena_PrimalItem_WeaponEmptyCryopod_Copy (Variables|/Script/ShooterGame.ShooterWeapon|GetAssociatedPrimalItem _asweap_empty_cryopod)))
    (if (.ReturnValue (Class|PrimalItem|GetCustomItemData _asarena_primal_item_weapon_empty_cryopod_copy "Dino"))
      (bind (_deployed _newlocation _failurereason) (Default|TryDeploy _asarena_primal_item_weapon_empty_cryopod_copy (Transformation|GetActorLocation) (Transformation|GetActorRotation) 0 self))
      (if _deployed
        (bind _returnvalue_2 (Class|VictoryCore|GetClassDefaultObject (.AsCharacter (Utilities|Casting|CastToCharacterClass (Utilities|Array|Get(acopy) (.CustomDataClasses (Utilities|Struct|BreakCustomItemData (.OutData (Class|PrimalItem|GetCustomItemData _asarena_primal_item_weapon_empty_cryopod_copy "Dino")))))))))
        (Default|DeploySuccess _asweap_empty_cryopod _newlocation (Transformation|GetActorRotation) (/ (Variables|/Script/Engine.CapsuleComponent|GetCapsuleRadius (Variables|/Script/Engine.Character|GetCapsuleComponent (.AsPrimal%20Dino%20Character (Utilities|Casting|CastToPrimalDinoCharacter _returnvalue_2)))) 1e+02))
        (else
          (Class|ShooterPlayerController|ClientServerNotificationSingle _asshooter_player_controller (Utilities|String|Append "Cannot Deploy: " _failurereason) "(R=1.000000,G=0.000000,B=0.016183,A=1.000000)" 1.0 3.0)
          (Default|DeployFailure _asweap_empty_cryopod (Transformation|GetActorLocation) (Transformation|GetActorRotation)))))))

(fn ConstructionScript)