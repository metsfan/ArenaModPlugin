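; Timed buff, named as a shorter Arena cryo cooldown, that starts a 20-second countdown on activation.
; Client and server ticks each count TimeLeft down, and the server deactivates the buff at zero.
; The HUD draws the remaining seconds to one decimal place.
; TimeLeft is written to generic time-remaining persistent data and read back on server BeginPlay when IsLoadingSaveGame is false.
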(fn ConstructionScript
  (|CallParentFunction))

(fn BuffTickClient
  (params (DeltaTime :type Float%20%28single-precision%29))
  (Variables|Default|SetTimeLeft (Math|Float|Max(Float) (- (Variables|Default|GetTimeLeft) DeltaTime) 0.0) false))

(fn BuffTickServer
  (params (DeltaTime :type Float%20%28single-precision%29))
  (Variables|Default|SetTimeLeft (Math|Float|Max(Float) (- (Variables|Default|GetTimeLeft) DeltaTime) 0.0) false)
  (if (Math|Float|NearlyEqual(Float) (Variables|Default|GetTimeLeft) 0.0 1e-06)
    (Class|PrimalBuff|BPDeactivate)))

(fn BPDrawBuffStatusHUD
  (params (HUD :type Shooter%20HUD%20Object%20Reference) (XPos :type Float%20%28single-precision%29) (YPos :type Float%20%28single-precision%29) (ScaleMult :type Float%20%28single-precision%29))
  (Class|Canvas|BPDrawTextCentered (Variables|/Script/Engine.HUD|GetCanvas HUD) (Variables|/Script/ShooterGame.ShooterHUD|GetNormalFont HUD) (Utilities|String|ToString(Text) (Utilities|Text|ToText(Float) (Variables|Default|GetTimeLeft) "HalfToEven" false true 1 324 1 1)) (+ XPos (* 32.0 ScaleMult)) (+ YPos (* 4e+01 ScaleMult)) 1.0 1.0 true false))

(fn ReceiveBeginPlay
  (|CallParentFunction)
  (if (Networking|IsServer)
    (bind _returnvalue (Class|VictoryCore|IsLoadingSaveGame))
    (if (not _returnvalue)
      (bind _asprimal_buff_persistent_data_generic_time_remaining (Utilities|Casting|CastToPrimalBuffPersistentData_GenericTimeRemaining (Variables|Default|GetMyBuffPersistentData)))
      (Variables|Default|SetTimeLeft (Variables|/Game/ScorchedEarth/CoreBlueprints/Buffs/PrimalBuffPersistentData_GenericTimeRemaining.PrimalBuffPersistentData_GenericTimeRemaining_C|GetTimeLeft _asprimal_buff_persistent_data_generic_time_remaining) false))))

(fn UpdateBuffPersistentData
  (bind _asprimal_buff_persistent_data_generic_time_remaining (Utilities|Casting|CastToPrimalBuffPersistentData_GenericTimeRemaining (Variables|Default|GetMyBuffPersistentData)))
  (Variables|/Game/ScorchedEarth/CoreBlueprints/Buffs/PrimalBuffPersistentData_GenericTimeRemaining.PrimalBuffPersistentData_GenericTimeRemaining_C|SetTimeLeft _asprimal_buff_persistent_data_generic_time_remaining (Variables|Default|GetTimeLeft)))

(fn BPActivated
  (params (ForInstigator :type Actor%20Object%20Reference))
  (Variables|Default|SetTimeLeft 2e+01 true))