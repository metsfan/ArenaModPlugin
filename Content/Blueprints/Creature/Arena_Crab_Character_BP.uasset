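; Arena variant of the crab creature that limits how it can grab and carry other characters.
; Enemy grabs start a five-second forced-drop timer, and released enemies receive a buff that blocks re-grabbing; same-team grabs require a riderless dino with no owning player.
; Losing the rider also drops carried characters.
; Lethal damage is forwarded to OnDinoLethalDamage, while the damage-adjust override passes values through unchanged.
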(fn ConstructionScript
  (|CallParentFunction))

(fn BPonLethalDamage
  (params (KillingDamage :type Float%20%28single-precision%29) (DamageEvent :type Damage%20Event%20Structure%20%28by%20ref%29) (Killer :type Controller%20Object%20Reference) (DamageCauser :type Actor%20Object%20Reference))
  (CallFunction|OnDinoLethalDamage self KillingDamage DamageEvent Killer DamageCauser)
  (return false))

(fn BPAllowCarryCharacter
  (params (checkCharacter :type Primal%20Character%20Object%20Reference))
  (LocalVariables|SetRet false)
  (Utilities|FlowControl|Sequence
    (:then_0
      (if (not (Class|PrimalCharacter|HasBuff checkCharacter "/ArenaMod/Buff_PreventCrabCarry.Buff_PreventCrabCarry_C" true))
        (Utilities|FlowControl|Sequence
          (:then_0
            (if (!= (Variables|/Script/Engine.Actor|GetTargetingTeam checkCharacter) (Variables|Default|GetTargetingTeam))
              (Utilities|FlowControl|Sequence
                (:then_0
                  (LocalVariables|SetRet true))
                (:then_1
                  (Utilities|Time|SetTimerbyFunctionName 0 "ForceDropCharacter" 5.0)))
              (else
                (bind _asprimal_dino_character (Utilities|Casting|CastToPrimalDinoCharacter checkCharacter))
                (LocalVariables|SetRet (and (== (Variables|/Script/ShooterGame.PrimalDinoCharacter|GetOwningPlayerID _asprimal_dino_character) 0) (not (Utilities|IsValid (Variables|/Script/ShooterGame.PrimalDinoCharacter|GetRider _asprimal_dino_character)))))))))))
    (:then_1
      (return (LocalVariables|GetRet)))))

(fn BPAdjustDamage
  (params (IncomingDamage :type Float%20%28single-precision%29) (TheDamageEvent :type Damage%20Event%20Structure) (EventInstigator :type Controller%20Object%20Reference) (DamageCauser :type Actor%20Object%20Reference) (bIsPointDamage :type Boolean) (PointHitInfo :type Hit%20Result%20Structure))
  (return IncomingDamage))

(fn ForceDropCharacter
  (CallFunction|ServerDropCharacters))

(fn BPNotifyClearRider
  (params (RiderClearing :type Shooter%20Character%20Object%20Reference))
  (|CallParentFunction RiderClearing)
  (CallFunction|ForceDropCharacter))

(fn BPNotifyClearPassenger
  (params (PassengerChar :type Primal%20Character%20Object%20Reference) (SeatIndex :type Integer))
  (if (!= (Variables|/Script/Engine.Actor|GetTargetingTeam PassengerChar) (Variables|Default|GetTargetingTeam))
    (Class|PrimalBuff|StaticAddBuff "/ArenaMod/Buff_PreventCrabCarry.Buff_PreventCrabCarry_C" PassengerChar 0 0 false)))