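; Arena variant of the Forest Kaiju creature character, built for the Arena mod game mode.
; Each tick, after parent logic, it forces TamedAggressionLevel to 0 while the creature is tamed.
; On lethal damage it reports itself and the killing PrimalCharacter to TestGameMode_ArenaMod through OnDinoDeath, then returns false.
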(event EventTick
  (params (DeltaSeconds :type Float%20%28single-precision%29))
  (|CallParentFunction DeltaSeconds)
  (Utilities|FlowControl|Sequence
    (:then_0
      (if (Class|PrimalDinoCharacter|BPIsTamed)
        (Variables|Default|SetTamedAggressionLevel 0 false)))))

(fn ConstructionScript
  (|CallParentFunction))

(fn BPonLethalDamage
  (params (KillingDamage :type Float%20%28single-precision%29) (DamageEvent :type Damage%20Event%20Structure%20%28by%20ref%29) (Killer :type Controller%20Object%20Reference) (DamageCauser :type Actor%20Object%20Reference))
  (Utilities|FlowControl|Sequence
    (:then_0
      (bind _astest_game_mode_arena_mod (Utilities|Casting|CastToTestGameMode_ArenaMod (Game|GetGameMode)))
      (bind _asprimal_character (Utilities|Casting|CastToPrimalCharacter Killer))
      (Default|OnDinoDeath _astest_game_mode_arena_mod self _asprimal_character))
    (:then_1
      (return false))))