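; Arena mod variant of the Basilisk creature that adjusts lethal damage, interaction and dive behavior.
; Lethal damage is passed to OnDinoLethalDamage, and the override returns false.
; Multi-use interactions reach the parent only for an arena player controller whose PersonalDino is this creature, or when the creature has no owning player ID.
; Dive initialization runs the parent logic, then clears IsUnderground.
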(fn ConstructionScript
  (|CallParentFunction))

(fn BPonLethalDamage
  (params (KillingDamage :type Float%20%28single-precision%29) (DamageEvent :type Damage%20Event%20Structure%20%28by%20ref%29) (Killer :type Controller%20Object%20Reference) (DamageCauser :type Actor%20Object%20Reference))
  (CallFunction|OnDinoLethalDamage self KillingDamage DamageEvent Killer DamageCauser)
  (return false))

(fn BPTryMultiUse
  (params (ForPC :type Player%20Controller%20Object%20Reference) (UseIndex :type Integer))
  (bind _asplayer_controller_blueprint_arena_mod (Utilities|Casting|CastToPlayerControllerBlueprint_ArenaMod ForPC))
  (if (or (== (Variables|/ArenaMod/PlayerControllerBlueprint_ArenaMod.PlayerControllerBlueprint_ArenaMod_C|GetPersonalDino _asplayer_controller_blueprint_arena_mod) self) (== (Variables|Default|GetOwningPlayerID) 0))
    (bind _returnvalue (|CallParentFunction ForPC UseIndex)))
  (return _returnvalue))

(fn InitializeDive
  (|CallParentFunction)
  (Variables|Default|SetisUnderground false true))