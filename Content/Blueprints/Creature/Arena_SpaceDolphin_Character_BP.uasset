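; Arena variant of the Space Dolphin creature character that adds a cooldown to the parent's loop maneuver.
; Starting a loop, Immelmann or otherwise, sets a cooldown flag that a timer clears, and CanLoop checks it alongside the parent's rules.
; Lethal damage is passed on through OnDinoLethalDamage with killer and damage details, then the override returns false.
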(fn ConstructionScript
  (|CallParentFunction))

(fn BPonLethalDamage
  (params (KillingDamage :type Float%20%28single-precision%29) (DamageEvent :type Damage%20Event%20Structure%20%28by%20ref%29) (Killer :type Controller%20Object%20Reference) (DamageCauser :type Actor%20Object%20Reference))
  (CallFunction|OnDinoLethalDamage self KillingDamage DamageEvent Killer DamageCauser)
  (return false))

(fn LoopCooldownExpire
  (Variables|Default|SetLoopOnCooldown false))

(fn StartLoop
  (params (Immelmann :type Boolean))
  (|CallParentFunction Immelmann)
  (Variables|Default|SetLoopOnCooldown true)
  (Utilities|Time|SetTimerbyFunctionName 0 "LoopCooldownExpire" (Variables|Default|GetLoopCooldownTime)))

(fn CanLoop
  (return (and (not (Variables|Default|GetLoopOnCooldown)) (|CallParentFunction))))

(fn BPKilledSomethingEvent
  (params (killedTarget :type Primal%20Character%20Object%20Reference)))