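; Desert Titan (kaiju) creature for the Arena mod that reports its death to the game mode.
; BPOnLethalDamage calls HandleDeathEvent and returns false.
; The event passes the Titan and killer to OnDinoDeath, only when the damage causer is a PrimalCharacter.
; It separately fetches the Capture the Artifact manager from the game mode and starts the Titan cooldown for its team.
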(event Custom|HandleDeathEvent
  (params (KillingDamage :type Float%20%28double-precision%29) (DamageEvent :type Damage%20Event%20Structure) (Killer :type Controller%20Object%20Reference) (DamageCauser :type Actor%20Object%20Reference))
  (bind _returnvalue (Game|GetGameMode))
  (bind _astest_game_mode_arena_mod (Utilities|Casting|CastToTestGameMode_ArenaMod _returnvalue))
  (Utilities|FlowControl|Sequence
    (:then_0
      (bind _asprimal_character (Utilities|Casting|CastToPrimalCharacter DamageCauser))
      (Default|OnDinoDeath _astest_game_mode_arena_mod self _asprimal_character))
    (:then_1
      (bind _returnvalue_2 (Default|GetSingletonGameManager _astest_game_mode_arena_mod "NewEnumerator4"))
      (bind _asgame_manager_capture_the_artifact (Utilities|Casting|CastToGameManager_CaptureTheArtifact _returnvalue_2))
      (Default|StartTitanCooldown _asgame_manager_capture_the_artifact (Variables|Default|GetTargetingTeam)))))

(fn ConstructionScript
  (|CallParentFunction))

(fn BPonLethalDamage
  (params (KillingDamage :type Float%20%28single-precision%29) (DamageEvent :type Damage%20Event%20Structure%20%28by%20ref%29) (Killer :type Controller%20Object%20Reference) (DamageCauser :type Actor%20Object%20Reference))
  (CallFunction|HandleDeathEvent KillingDamage DamageEvent Killer DamageCauser)
  (return false))