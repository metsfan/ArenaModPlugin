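; Arena variant of the Gigant rage buff that scales the damage seen by the parent buff's logic according to damage type.
; BuffAdjustDamage checks the damage type against RageNerfDamageTypes, including subclasses, and takes the multiplier at the same index in RageNerfDamageAmount, with the last match winning.
; The scaled value goes only to the parent implementation; the function returns the original damage unchanged.
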(fn ConstructionScript
  (|CallParentFunction))

(fn BuffAdjustDamage
  (params (Damage :type Float%20%28single-precision%29) (HitInfo :type Hit%20Result%20Structure%20%28by%20ref%29) (EventInstigator :type Controller%20Object%20Reference) (TheDamageCauser :type Actor%20Object%20Reference) (TheDamgeType :type Damage%20Type%20Class%20Reference))
  (LocalVariables|SetRageDamageMultiplier 1.0)
  (Utilities|FlowControl|Sequence
    (:then_0
      (for (_array_element _array_index) (Variables|Default|GetRageNerfDamageTypes)
        (if (Utilities|ClassIsChildOf TheDamgeType _array_element)
          (LocalVariables|SetRageDamageMultiplier (Utilities|Array|Get(acopy) (Variables|Default|GetRageNerfDamageAmount) _array_index)))))
    (:then_1
      (|CallParentFunction (* Damage (LocalVariables|GetRageDamageMultiplier)) HitInfo EventInstigator TheDamageCauser TheDamgeType))
    (:then_2
      (return Damage))))