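; Arena variant of the Paracer (Paraceratherium) creature, with a platform saddle build area.
; On lethal damage it passes the hit details to OnDinoLethalDamage and returns false.
; Tamed setup shows the platform block and resizes the saddle build area to the configured extents.
; Server-side loading of the saved "ParacerPlatform" structures is present but disconnected, so BeginPlay only runs the parent logic.
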(event EventBeginPlay
  (|CallParentFunction))

(fn ConstructionScript
  (|CallParentFunction))

(fn BPonLethalDamage
  (params (KillingDamage :type Float%20%28single-precision%29) (DamageEvent :type Damage%20Event%20Structure%20%28by%20ref%29) (Killer :type Controller%20Object%20Reference) (DamageCauser :type Actor%20Object%20Reference))
  (CallFunction|OnDinoLethalDamage self KillingDamage DamageEvent Killer DamageCauser)
  (return false))

(fn BPSetupTamed
  (params (bWasJustTamed :type Boolean))
  (|CallParentFunction bWasJustTamed)
  (Rendering|SetVisibility (Variables|Default|GetPlatformBlock) true false)
  (Components|Box|SetBoxExtent (Variables|Default|GetPlatformSaddleBuildArea) (Variables|Default|GetPlatformBuildExtents) true))