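; Creature buff, a no-friendly variant of an Encapsulated effect, that strips itself from allies of the dino that caused it.
; On setup it compares the instigator's targeting team with that of the buff damage causer.
; For a same-team character other than that dino or its rider, it deactivates buffs of its own class, subclasses included.
; If the causer is not a dino, the buff is left in place.
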(fn ConstructionScript
  (|CallParentFunction))

(fn BPSetupforInstigator
  (params (ForInstigator :type Actor%20Object%20Reference))
  (bind _buffdamagecauser (Variables|Default|GetBuffDamageCauser))
  (if (== (Variables|/Script/Engine.Actor|GetTargetingTeam ForInstigator) (Variables|/Script/Engine.Actor|GetTargetingTeam _buffdamagecauser))
    (bind _asprimal_dino_character (Utilities|Casting|CastToPrimalDinoCharacter _buffdamagecauser))
    (if (and (!= ForInstigator (Variables|/Script/ShooterGame.PrimalDinoCharacter|GetRider _asprimal_dino_character)) (!= ForInstigator _buffdamagecauser))
      (bind _asprimal_character (Utilities|Casting|CastToPrimalCharacter ForInstigator))
      (Class|PrimalCharacter|DeactivateBuffs _asprimal_character (.AsPrimal%20Buff (Utilities|Casting|CastToPrimalBuffClass (Utilities|GetClass self))) 0 false))))