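; Arena creature buff for Capture the Artifact that rewards mounted dinos and cleans up idle ones.
; A one-second timer sets damage-taken and melee multipliers by rider presence and copies the rider's active team buffs, removed on EndPlay.
; Idle time since last mounted drives unclaiming or destruction, in both the timer and server tick.
; It also blocks Tek Wyvern breath stun on high-drag-weight dinos, applying another buff instead.
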(event Custom|CheckBuffTick
  (bind _instigator (Variables|Default|GetInstigator))
  (bind _asprimal_dino_character (Utilities|Casting|CastToPrimalDinoCharacter _instigator))
  (bind _rider (Variables|/Script/ShooterGame.PrimalDinoCharacter|GetRider _asprimal_dino_character))
  (bind _returnvalue (Default|GetSingletonGameManager (.AsTest%20Game%20Mode%20Arena%20Mod (Utilities|Casting|CastToTestGameMode_ArenaMod (Game|GetGameMode))) "NewEnumerator4"))
  (bind _asgame_manager_capture_the_artifact (Utilities|Casting|CastToGameManager_CaptureTheArtifact _returnvalue))
  (Utilities|FlowControl|Sequence
    (:then_0
      (CallFunction|UpdateRiderBonus _asgame_manager_capture_the_artifact))
    (:then_1
      (Utilities|IsValid _rider
        (:Is%20Valid
          (bind _team (Default|GetPrimalCharacterTeam _asgame_manager_capture_the_artifact _asprimal_dino_character))
          (for _array_element (Variables|/ArenaMod/GameManager/GameManager_CaptureTheArtifact.GameManager_CaptureTheArtifact_C|GetTeamBuffs _asgame_manager_capture_the_artifact)
            (bind _asctateam_buff (Utilities|Casting|CastToCTATeamBuff _array_element))
            (if (== _team (Variables|/ArenaMod/GameManager/CTA/TeamBuff/CTATeamBuff.CTATeamBuff_C|GetTeam _asctateam_buff))
              (if (Math|Boolean|ANDBoolean (not (Class|PrimalCharacter|HasBuff _asprimal_dino_character (Variables|/ArenaMod/GameManager/CTA/TeamBuff/CTATeamBuff.CTATeamBuff_C|GetBuffClass _asctateam_buff) true)) (Class|PrimalCharacter|HasBuff _rider (Variables|/ArenaMod/GameManager/CTA/TeamBuff/CTATeamBuff.CTATeamBuff_C|GetBuffClass _asctateam_buff) true) (> (Variables|/ArenaMod/GameManager/CTA/TeamBuff/CTATeamBuff.CTATeamBuff_C|GetTimeRemaining _asctateam_buff) 0.0))
                (Utilities|FlowControl|Sequence
                  (:then_0
                    (bind _returnvalue_2 (Class|PrimalBuff|StaticAddBuff (Variables|/ArenaMod/GameManager/CTA/TeamBuff/CTATeamBuff.CTATeamBuff_C|GetBuffClass _asctateam_buff) _asprimal_dino_character 0 0 false))
                    (Class|PrimalBuff|ExtendBuffTime _returnvalue_2 (Variables|/ArenaMod/GameManager/CTA/TeamBuff/CTATeamBuff.CTATeamBuff_C|GetTimeRemaining _asctateam_buff)))
                  (:then_1
                    (Utilities|Array|Add (Variables|Default|GetAddedBuffs) (Variables|/ArenaMod/GameManager/CTA/TeamBuff/CTATeamBuff.CTATeamBuff_C|GetBuffClass _asctateam_buff))))))))))))

(event EventBuffTickServer
  (params (DeltaTime :type Float%20%28single-precision%29))
  (bind _returnvalue (Utilities|Time|GetRealTimeSeconds))
  (bind _lastmountedtime (Variables|Default|GetLastMountedTime))
  (bind _returnvalue_2 (- _returnvalue _lastmountedtime))
  (Utilities|FlowControl|Sequence
    (:then_0
      (bind _asprimal_dino_character (Utilities|Casting|CastToPrimalDinoCharacter (Variables|Default|GetInstigator)))
      (Utilities|IsValid (Variables|/Script/ShooterGame.PrimalDinoCharacter|GetRider _asprimal_dino_character)
        (:Is%20Not%20Valid
          (if (not (or (Variables|/Script/ShooterGame.PrimalDinoCharacter|GetbIsInTurretMode _asprimal_dino_character) (== (Utilities|GetClass _asprimal_dino_character) 0)))
            (if (>= _returnvalue_2 (Variables|Default|GetMaxIdleTimeDespawn))
              (if (not (Class|PrimalCharacter|HasBuff _asprimal_dino_character 0 false))
                (Actor|DestroyActor _asprimal_dino_character))
              (elif (>= _returnvalue_2 (Variables|Default|GetMaxIdleTimeUnclaim))
                (CallFunction|UnclaimPersonalDino _asprimal_dino_character)))))))))

(event EventEndPlay
  (params (EndPlayReason :type EEndPlayReason%20Enum :default "Destroyed"))
  (|CallParentFunction EndPlayReason)
  (for _array_element (Variables|Default|GetAddedBuffs)
    (Class|PrimalCharacter|DeactivateBuffs (.AsPrimal%20Dino%20Character (Utilities|Casting|CastToPrimalDinoCharacter (Variables|Default|GetInstigator))) _array_element 0 true)))

(event EventBeginPlay
  (|CallParentFunction)
  (Utilities|Time|SetTimerbyEvent (delegate Custom|CheckBuffTick) 1.0 true)
  (Variables|Default|SetLastMountedTime (Utilities|Time|GetRealTimeSeconds)))

(fn ConstructionScript
  (|CallParentFunction))

(fn UpdateRiderBonus
  (params (GameManager :type Game%20Manager%20Capture%20the%20Artifact%20Object%20Reference))
  (bind _instigator (Variables|Default|GetInstigator))
  (Utilities|FlowControl|Sequence
    (:then_1
      (bind _targetingteam (Default|GetAdvantageTeam GameManager))
      (if (== _targetingteam (Variables|Default|GetTargetingTeam))
        (LocalVariables|SetAdvantageMultiplier (* 0 0.05))))
    (:then_2
      (Utilities|IsValid (Variables|/Script/ShooterGame.PrimalDinoCharacter|GetRider (.AsPrimal%20Dino%20Character (Utilities|Casting|CastToPrimalDinoCharacter _instigator)))
        (:Is%20Valid
          (Variables|Default|SetReceiveDamageMultiplier 0.5)
          (Variables|Default|SetMeleeDamageMultiplier (+ (LocalVariables|GetAdvantageMultiplier) 1.5))
          (Variables|Default|SetLastMountedTime (Utilities|Time|GetRealTimeSeconds)))
        (:Is%20Not%20Valid
          (Variables|Default|SetReceiveDamageMultiplier 1.0)
          (Variables|Default|SetMeleeDamageMultiplier 1.0))))
    (:then_3
      (if (>= (- (Utilities|Time|GetRealTimeSeconds) (Variables|Default|GetLastMountedTime)) (Variables|Default|GetMaxIdleTimeUnclaim))
        (Actor|DestroyActor _instigator)))))

(fn BPPreventAddingOtherBuff
  (params (anotherBuffClass :type Primal%20Buff%20Class%20Reference))
  (Utilities|FlowControl|Sequence
    (:then_0
      (if (== anotherBuffClass "/Game/Genesis2/CoreBlueprints/Buffs/Buff_TekWyvern_BreathStun.Buff_TekWyvern_BreathStun_C")
        (bind _asprimal_dino_character (Utilities|Casting|CastToPrimalDinoCharacter (Game|GetInstigator)))
        (if (>= (Variables|/Script/ShooterGame.PrimalCharacter|GetDragWeight _asprimal_dino_character) 5e+02)
          (LocalVariables|SetRet true)
          (if (not (Class|PrimalCharacter|HasBuff _asprimal_dino_character 0 false))
            (Class|PrimalBuff|StaticAddBuff 0 _asprimal_dino_character 0 0 false)))))
    (:then_1
      (return (LocalVariables|GetRet)))))