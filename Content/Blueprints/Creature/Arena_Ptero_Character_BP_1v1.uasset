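; Pteranodon creature variant for a 1v1 arena, extending its parent character Blueprint.
; Every tick it runs the parent logic, then forces TamedAggressionLevel to zero while the creature is tamed.
; BPAdjustDamage scales all incoming damage by GlobalDamageModifier, regardless of damage type or source.
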(event EventTick
  (params (DeltaSeconds :type Float%20%28single-precision%29))
  (|CallParentFunction DeltaSeconds)
  (Utilities|FlowControl|Sequence
    (:then_0
      (if (Class|PrimalDinoCharacter|BPIsTamed)
        (Variables|Default|SetTamedAggressionLevel 0 false)))))

(fn ConstructionScript
  (|CallParentFunction))

(fn BPAdjustDamage
  (params (IncomingDamage :type Float%20%28single-precision%29) (TheDamageEvent :type Damage%20Event%20Structure) (EventInstigator :type Controller%20Object%20Reference) (DamageCauser :type Actor%20Object%20Reference) (bIsPointDamage :type Boolean) (PointHitInfo :type Hit%20Result%20Structure))
  (return (* IncomingDamage (Variables|Default|GetGlobalDamageModifier))))