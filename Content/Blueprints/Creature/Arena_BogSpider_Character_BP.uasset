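; Arena variant of the Bog Spider creature that adds team rules to its carry and bio-grapple abilities.
; Overrides extend the parent checks to reject same-team targets, and grappling also requires a valid rider.
; Clearing the rider releases any ensnared character.
; Lethal damage is forwarded to OnDinoLethalDamage with the killer details, and the override returns false.
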(fn ConstructionScript
  (|CallParentFunction))

(fn BPonLethalDamage
  (params (KillingDamage :type Float%20%28single-precision%29) (DamageEvent :type Damage%20Event%20Structure%20%28by%20ref%29) (Killer :type Controller%20Object%20Reference) (DamageCauser :type Actor%20Object%20Reference))
  (CallFunction|OnDinoLethalDamage self KillingDamage DamageEvent Killer DamageCauser)
  (return false))

(fn BPAllowCarryCharacter
  (params (checkCharacter :type Primal%20Character%20Object%20Reference))
  (bind _returnvalue (|CallParentFunction checkCharacter))
  (return (and _returnvalue (!= (Variables|/Script/Engine.Actor|GetTargetingTeam checkCharacter) (Variables|Default|GetTargetingTeam)))))

(fn IsValidBioGrappleTarget
  (params (ForGrappleTarget :type Primal%20Character%20Object%20Reference) (bForStart :type Boolean) (bPreventTraces :type Boolean))
  (bind _bresult (|CallParentFunction ForGrappleTarget bForStart bPreventTraces))
  (return (Math|Boolean|ANDBoolean _bresult (!= (Variables|/Script/Engine.Actor|GetTargetingTeam ForGrappleTarget) (Variables|Default|GetTargetingTeam)) (Utilities|IsValid (Variables|Default|GetRider)))))

(fn BPNotifyClearRider
  (params (RiderClearing :type Shooter%20Character%20Object%20Reference))
  (|CallParentFunction RiderClearing)
  (CallFunction|ReleaseEnsnaredChar))