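; Arena variant of the Megalosaurus creature character, adapted for an arena game mode.
; It applies a rider bonus buff to itself when a rider mounts and deactivates that buff when the rider leaves.
; On lethal damage it reports the death to the arena game mode, crediting the damage causer as killer if it is a character, and returns false.
; It also disallows carrying other characters.
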(fn ConstructionScript
  (|CallParentFunction))

(fn BPNotifySetRider
  (params (RiderSetting :type Shooter%20Character%20Object%20Reference))
  (Utilities|FlowControl|Sequence
    (:then_0
      (Class|PrimalBuff|StaticAddBuff "/Game/Mods/ArenaMod/Blueprints/Creature/Arena_Buff_RiderBonus.Arena_Buff_RiderBonus_C" self 0 0 false))))

(fn BPNotifyClearRider
  (params (RiderClearing :type Shooter%20Character%20Object%20Reference))
  (Utilities|FlowControl|Sequence
    (:then_0
      (Class|PrimalCharacter|DeactivateBuffs "/Game/Mods/ArenaMod/Blueprints/Creature/Arena_Buff_RiderBonus.Arena_Buff_RiderBonus_C" 0 false))))

(fn BPonLethalDamage
  (params (KillingDamage :type Float%20%28single-precision%29) (DamageEvent :type Damage%20Event%20Structure%20%28by%20ref%29) (Killer :type Controller%20Object%20Reference) (DamageCauser :type Actor%20Object%20Reference))
  (Utilities|FlowControl|Sequence
    (:then_0
      (bind _astest_game_mode_arena_mod (Utilities|Casting|CastToTestGameMode_ArenaMod (Game|GetGameMode)))
      (bind _asprimal_character (Utilities|Casting|CastToPrimalCharacter DamageCauser))
      (Default|OnDinoDeath _astest_game_mode_arena_mod self _asprimal_character))
    (:then_1
      (return false))))

(fn BPAllowCarryCharacter
  (params (checkCharacter :type Primal%20Character%20Object%20Reference))
  (return false))