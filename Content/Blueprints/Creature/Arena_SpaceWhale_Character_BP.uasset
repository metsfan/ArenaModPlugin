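; Arena variant of the Space Whale creature that disables hyperdrive by always refusing its use check.
; On lethal damage it passes the hit details to OnDinoLethalDamage and returns false.
; Local bomb targeting requests require a rider with a ShooterPlayerState, deactivate the rider's targeting buff when turning off, then send the mode to the server.
; The client-side code that would add that buff is left unconnected.
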(fn ConstructionScript
  (|CallParentFunction))

(fn BPonLethalDamage
  (params (KillingDamage :type Float%20%28single-precision%29) (DamageEvent :type Damage%20Event%20Structure%20%28by%20ref%29) (Killer :type Controller%20Object%20Reference) (DamageCauser :type Actor%20Object%20Reference))
  (CallFunction|OnDinoLethalDamage self KillingDamage DamageEvent Killer DamageCauser)
  (return false))

(fn LocalRequestBombTargeting
  (params (NewBombTargetingMode :type Boolean))
  (bind _rider (Variables|Default|GetRider))
  (bind _bombtargettingbuff (Variables|Default|GetBombTargettingBuff))
  (bind _returnvalue (Class|PrimalCharacter|GetBuff _rider _bombtargettingbuff))
  (Utilities|Casting|CastToShooterPlayerState (Variables|/Script/Engine.Pawn|GetPlayerState _rider))
  (Utilities|FlowControl|Sequence
    (:then_0
      (if (not NewBombTargetingMode)
        (Utilities|IsValid _returnvalue
          (:Is%20Valid
            (Components|Activation|Deactivate _returnvalue)))))
    (:then_1
      (CallFunction|ServerRequestSetBombTargetingMode NewBombTargetingMode))))

(fn AllowedtoUseHyperdrive
  (params (CheckTimer :type Boolean) (Target :type Vector :default "0, 0, 0"))
  (return false))