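; Reaper creature character for an arena mod, adjusting the creature's behavior for that game mode.
; On server BeginPlay it applies an Aberration bonus buff when the TestGameMode_ArenaMod next CTA map matches one specific enum value.
; Lethal damage is reported through OnDinoLethalDamage and returns false, while the damage adjustment hook passes damage through unchanged.
; Multi-use skips the parent handler for one reserved index and forwards all others as index zero.
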(event EventBeginPlay
  (|CallParentFunction)
  (if (Networking|IsServer)
    (bind _astest_game_mode_arena_mod (Utilities|Casting|CastToTestGameMode_ArenaMod (Game|GetGameMode)))
    (if (Utilities|Enum|Equal(Enum) (Variables|/ArenaMod/TestGameMode_ArenaMod.TestGameMode_ArenaMod_C|GetNextCTAMap _astest_game_mode_arena_mod) "NewEnumerator2")
      (Class|PrimalBuff|StaticAddBuff "/Game/Mods/ArenaMod/Blueprints/Creature/Buff_ReaperAbBonus.Buff_ReaperAbBonus_C" self 0 0 false))))

(fn ConstructionScript
  (|CallParentFunction))

(fn BPAdjustDamage
  (params (IncomingDamage :type Float%20%28single-precision%29) (TheDamageEvent :type Damage%20Event%20Structure) (EventInstigator :type Controller%20Object%20Reference) (DamageCauser :type Actor%20Object%20Reference) (bIsPointDamage :type Boolean) (PointHitInfo :type Hit%20Result%20Structure))
  (return IncomingDamage))

(fn BPonLethalDamage
  (params (KillingDamage :type Float%20%28single-precision%29) (DamageEvent :type Damage%20Event%20Structure%20%28by%20ref%29) (Killer :type Controller%20Object%20Reference) (DamageCauser :type Actor%20Object%20Reference))
  (CallFunction|OnDinoLethalDamage self KillingDamage DamageEvent Killer DamageCauser)
  (return false))

(fn BPTryMultiUse
  (params (ForPC :type Player%20Controller%20Object%20Reference) (UseIndex :type Integer))
  (if (== UseIndex 7789)
    _
    (else
      (bind _returnvalue (|CallParentFunction ForPC 0))))
  (return _returnvalue))