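; Buff_DeathSentence is a creature buff that drains the instigating dino's health to kill it over a set time.
; On the server, one second after BeginPlay, it reads the dino's current health.
; It then sets a negative per-second Health value of that amount divided by TimeToKill.
; Instigators that are not PrimalDinoCharacters are ignored.
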(event EventBeginPlay
  (if (Networking|IsServer)
    (Utilities|FlowControl|Delay 0 1.0)
    (bind _asprimal_dino_character (Utilities|Casting|CastToPrimalDinoCharacter (Variables|Default|GetInstigator)))
    (Class|PrimalBuff|SetValuetoAddPerSecond "Health" (* (* (Class|PrimalCharacterStatusComponent|BPGetCurrentStatusValue (Variables|/Script/ShooterGame.PrimalCharacter|GetMyCharacterStatusComponent _asprimal_dino_character) "Health") (/ 1.0 (Variables|Default|GetTimeToKill))) -1.0))))

(fn ConstructionScript)