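; Event Queen variant of the female Xenomorph creature, which impregnates the character it carries and then removes itself.
; The impregnate anim notify runs on the server, giving a living carried victim the Super Reaper pregnancy buff and dropping health above 1 down to 1.
; The release notify calls the parent, then starts a ten-second timer that destroys the queen if it is still alive.
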(event Custom|KillAfterPreg
  (if (not (Class|PrimalActor|IsDead))
    (Actor|DestroyActor)))

(event EventAnimNotifyImpregnateRelease
  (|CallParentFunction)
  (Utilities|Time|SetTimerbyEvent (delegate Custom|KillAfterPreg) 1e+01))

(event EventAnimNotifyImpregnate
  (bind _carriedcharacter (Variables|Default|GetCarriedCharacter))
  (bind _mycharacterstatuscomponent (Variables|/Script/ShooterGame.PrimalCharacter|GetMyCharacterStatusComponent _carriedcharacter))
  (if (Networking|IsServer)
    (if (and (Utilities|IsValid _carriedcharacter) (not (Variables|/Script/ShooterGame.PrimalCharacter|GetbIsDead _carriedcharacter)))
      (Class|PrimalBuff|StaticAddBuff "/ArenaMod/GameManager/CTA/Event/Buff_SuperReaper_Preggers.Buff_SuperReaper_Preggers_C" _carriedcharacter 0 self false)
      (if (> (Class|PrimalCharacterStatusComponent|BPGetCurrentStatusValue _mycharacterstatuscomponent "Health") 1.0)
        (Class|PrimalCharacterStatusComponent|ModifyCurrentStatusValue _mycharacterstatuscomponent "Health" 1.0 false false true true 0 false false)))))

(fn ConstructionScript
  (|CallParentFunction))