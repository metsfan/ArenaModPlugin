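; Component on a dino that lets players claim or unclaim it as their personal dino in the Arena mod.
; It builds multi-use menu entries from the owner state: unclaim, a personally-owned notice, or claim with any remaining cooldown shown.
; Selections are forwarded to the Arena player controller's claim and unclaim functions.
; Ownership comes from the dino's OwningPlayerID, compared against the player's linked ID.
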(fn GetDinoMultiuseOptions
  (params (Player :type Player%20Controller%20Object%20Reference) (Entries :type Array%20of%20Multi%20Use%20Entry%20Structures))
  (Utilities|Casting|CastToPrimalDinoCharacter (Components|GetOwner))
  (bind _asplayer_controller_blueprint_arena_mod (Utilities|Casting|CastToPlayerControllerBlueprint_ArenaMod Player))
  (Utilities|FlowControl|Sequence
    (:then_0
      (if (CallFunction|HasPersonalOwner)
        (if (CallFunction|IsPersonalOwner _asplayer_controller_blueprint_arena_mod)
          (Utilities|FlowControl|Sequence
            (:then_0
              (Utilities|Array|Add Entries (Utilities|Struct|MakeMultiUseEntry 0 "Unclaim Personal Dino" 9901 0 false false false false false false false false false false false false false false 0 false 0 "(B=175,G=175,R=175,A=255)" "(B=255,G=255,R=255,A=255)" 3.0 3.0))))
          (else
            (Utilities|FlowControl|Sequence
              (:then_0
                (bind _returnvalue (Class|ShooterPlayerController|GetPlayerCharacterName _asplayer_controller_blueprint_arena_mod))
                (Utilities|Array|Add Entries (Utilities|Struct|MakeMultiUseEntry 0 (Utilities|String|ToString(Text) (Utilities|Text|FormatText "This dino is personally owned by {name}" (Utilities|Text|ToText(String) _returnvalue))) 0 0 false true true))))))
        (elif (<= (Variables|/ArenaMod/PlayerControllerBlueprint_ArenaMod.PlayerControllerBlueprint_ArenaMod_C|GetTimeUntilPersonalTame _asplayer_controller_blueprint_arena_mod) 0.0)
          (Utilities|Array|Add Entries (Utilities|Struct|MakeMultiUseEntry 0 "Claim Personal Dino" 9900 0 false false false false false false false false false false false false false false 0 false 0 "(B=175,G=175,R=175,A=255)" "(B=255,G=255,R=255,A=255)" 3.0))
          (else
            (bind _returnvalue_2 (Class|VictoryCore|FormatasTime (Math|Float|Floor (Variables|/ArenaMod/PlayerControllerBlueprint_ArenaMod.PlayerControllerBlueprint_ArenaMod_C|GetTimeUntilPersonalTame _asplayer_controller_blueprint_arena_mod)) false false true))
            (Utilities|Array|Add Entries (Utilities|Struct|MakeMultiUseEntry 0 (Utilities|String|ToString(Text) (Utilities|Text|FormatText "Claim Personal Dino {time}" (Utilities|Text|ToText(String) _returnvalue_2))) -1 0 false true false false false false false false false false false false false false 0 false 0 "(B=175,G=175,R=175,A=255)" "(B=255,G=255,R=255,A=255)" 3.0))))))
    (:then_1
      (return Entries))))

(fn DoTryMultiuseOptions
  (params (Player :type Player%20Controller%20Object%20Reference) (Index :type Integer))
  (bind _asprimal_dino_character (Utilities|Casting|CastToPrimalDinoCharacter (Components|GetOwner)))
  (bind _asplayer_controller_blueprint_arena_mod (Utilities|Casting|CastToPlayerControllerBlueprint_ArenaMod Player))
  (Utilities|FlowControl|Sequence
    (:then_0
      (LocalVariables|SetIsHandled true))
    (:then_1
      (switch int Index
        (:Default
          (LocalVariables|SetIsHandled false))
        (:9900
          (Utilities|FlowControl|Sequence
            (:then_0
              (Default|ClaimPersonalDino _asplayer_controller_blueprint_arena_mod _asprimal_dino_character))))
        (:9901
          (Utilities|FlowControl|Sequence
            (:then_0
              (Default|UnclaimPersonalDino _asplayer_controller_blueprint_arena_mod))))))
    (:then_2
      (return (LocalVariables|GetIsHandled)))))

(fn IsPersonalOwner
  (params (Player :type Player%20Controller%20Blueprint%20Arena%20Mod%20Object%20Reference))
  (bind _asprimal_dino_character (Utilities|Casting|CastToPrimalDinoCharacter (Components|GetOwner)))
  (bind _returnvalue (Class|ShooterPlayerController|LinkedPlayerIDString Player))
  (return (and (Utilities|Enum|Equal(Enum) _returnvalue (Utilities|String|ToString(Integer) (Variables|/Script/ShooterGame.PrimalDinoCharacter|GetOwningPlayerID _asprimal_dino_character))) (CallFunction|HasPersonalOwner))))

(fn HasPersonalOwner
  (bind _asprimal_dino_character (Utilities|Casting|CastToPrimalDinoCharacter (Components|GetOwner)))
  (return (> (Variables|/Script/ShooterGame.PrimalDinoCharacter|GetOwningPlayerID _asprimal_dino_character) 0)))