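; Creature buff for the Arena mod that lets team members claim a dino as their personal dino through its multi-use menu.
; Menu entries depend on OwningPlayerID, rider presence, the player's personal-tame cooldown and an optional exclusive claimer.
; Selected uses call claim or unclaim on the mod's player controller.
; AllowExclusiveClaimer reserves claiming for one player ID, then clears it after a timeout, forcing a net update each time.
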(event Custom|AllowExclusiveClaimer
  (params (Player :type Player%20Controller%20Blueprint%20Arena%20Mod%20Object%20Reference))
  (Utilities|FlowControl|Sequence
    (:then_0
      (bind _returnvalue (Class|ShooterPlayerController|LinkedPlayerIDString Player))
      (Variables|Default|SetExclusiveClaimer _returnvalue false)
      (Networking|ForceNetUpdate))
    (:then_1
      (Utilities|FlowControl|Delay 0 (Variables|Default|GetExclusiveClaimTimeout))
      (Variables|Default|SetExclusiveClaimer "" false)
      (Networking|ForceNetUpdate))))

(fn ConstructionScript
  (|CallParentFunction))

(fn BPGetMultiUseEntries
  (params (ForPC :type Player%20Controller%20Object%20Reference) (MultiUseEntries :type Array%20of%20Multi%20Use%20Entry%20Structures))
  (bind _exclusiveclaimer (Variables|Default|GetExclusiveClaimer))
  (bind _multiusecomponent (Variables|Default|GetMultiUseComponent))
  (bind _asprimal_dino_character (Utilities|Casting|CastToPrimalDinoCharacter (Game|GetInstigator)))
  (bind _asplayer_controller_blueprint_arena_mod (Utilities|Casting|CastToPlayerControllerBlueprint_ArenaMod ForPC))
  (bind _returnvalue (Class|ShooterPlayerController|LinkedPlayerIDString _asplayer_controller_blueprint_arena_mod))
  (Utilities|FlowControl|Sequence
    (:then_0
      (if (and (== (Variables|/Script/Engine.Actor|GetTargetingTeam _asprimal_dino_character) (Variables|/Script/Engine.Actor|GetTargetingTeam _asplayer_controller_blueprint_arena_mod)) (not (Utilities|IsValid (Variables|/Script/ShooterGame.PrimalDinoCharacter|GetRider _asprimal_dino_character))))
        (if (CallFunction|HasPersonalOwner)
          (if (CallFunction|IsPersonalOwner _asplayer_controller_blueprint_arena_mod)
            (Utilities|FlowControl|Sequence
              (:then_0
                (Utilities|Array|Add MultiUseEntries (Utilities|Struct|MakeMultiUseEntry _multiusecomponent "Unclaim Personal Dino" 9901 0 false false false false false false false false false false false false false false 0 false 0 "(B=175,G=175,R=175,A=255)" "(B=255,G=255,R=255,A=255)" 3.0 3.0))))
            (else
              (Utilities|FlowControl|Sequence
                (:then_0
                  (Utilities|Array|Clear MultiUseEntries)
                  (Utilities|Array|Add MultiUseEntries (Utilities|Struct|MakeMultiUseEntry _multiusecomponent "This dino is personally owned" 0 0 false true true))))))
          (elif (<= (Variables|/ArenaMod/PlayerControllerBlueprint_ArenaMod.PlayerControllerBlueprint_ArenaMod_C|GetTimeUntilPersonalTame _asplayer_controller_blueprint_arena_mod) 0.0)
            (if (or (== (Utilities|String|Len _exclusiveclaimer) 0) (Utilities|Enum|Equal(Enum) _exclusiveclaimer _returnvalue))
              (Utilities|Array|Add MultiUseEntries (Utilities|Struct|MakeMultiUseEntry _multiusecomponent "Claim Personal Dino" 9900 -1 false false false false false false false false false false false false false false 0 false 0 "(B=175,G=175,R=175,A=255)" "(B=255,G=255,R=255,A=255)" 0.5 0.5))
              (else
                (Utilities|FlowControl|Sequence
                  (:then_0
                    (Utilities|Array|Clear MultiUseEntries))
                  (:then_1
                    (Utilities|Array|Add MultiUseEntries (Utilities|Struct|MakeMultiUseEntry _multiusecomponent "You cannot claim this dino yet" 0 0 false true true))))))
            (else
              (bind _returnvalue_2 (Class|VictoryCore|FormatasTime (Math|Float|Floor (Variables|/ArenaMod/PlayerControllerBlueprint_ArenaMod.PlayerControllerBlueprint_ArenaMod_C|GetTimeUntilPersonalTame _asplayer_controller_blueprint_arena_mod)) false false true))
              (Utilities|Array|Add MultiUseEntries (Utilities|Struct|MakeMultiUseEntry _multiusecomponent (Utilities|String|ToString(Text) (Utilities|Text|FormatText "Claim Personal Dino {time}" (Utilities|Text|ToText(String) _returnvalue_2))) -1 -1 false true false false false false false false false false false false false false 0 false 0 "(B=175,G=175,R=175,A=255)" "(B=255,G=255,R=255,A=255)" 3.0)))))))
    (:then_1
      (return MultiUseEntries))))

(fn BPTryMultiUse
  (params (ForPC :type Player%20Controller%20Object%20Reference) (UseIndex :type Integer))
  (bind _asprimal_dino_character (Utilities|Casting|CastToPrimalDinoCharacter (Game|GetInstigator)))
  (bind _asplayer_controller_blueprint_arena_mod (Utilities|Casting|CastToPlayerControllerBlueprint_ArenaMod ForPC))
  (Utilities|FlowControl|Sequence
    (:then_0
      (LocalVariables|SetIsHandled true))
    (:then_1
      (switch int UseIndex
        (:Default
          (LocalVariables|SetIsHandled false))
        (:9900
          (Utilities|FlowControl|Sequence
            (:then_0
              (Default|ClaimPersonalDino _asplayer_controller_blueprint_arena_mod _asprimal_dino_character))))
        (:9901
          (Utilities|FlowControl|Sequence
            (:then_0
              (Default|UnclaimPersonalDino _asplayer_controller_blueprint_arena_mod))))))
    (:then_2
      (return (LocalVariables|GetIsHandled)))))

(fn HasPersonalOwner
  (bind _asprimal_dino_character (Utilities|Casting|CastToPrimalDinoCharacter (Game|GetInstigator)))
  (return (> (Variables|/Script/ShooterGame.PrimalDinoCharacter|GetOwningPlayerID _asprimal_dino_character) 0)))

(fn IsPersonalOwner
  (params (Player :type Player%20Controller%20Blueprint%20Arena%20Mod%20Object%20Reference))
  (bind _asprimal_dino_character (Utilities|Casting|CastToPrimalDinoCharacter (Game|GetInstigator)))
  (bind _returnvalue (Class|ShooterPlayerController|LinkedPlayerIDString Player))
  (return (and (Utilities|Enum|Equal(Enum) _returnvalue (Utilities|String|ToString(Integer) (Variables|/Script/ShooterGame.PrimalDinoCharacter|GetOwningPlayerID _asprimal_dino_character))) (CallFunction|HasPersonalOwner))))