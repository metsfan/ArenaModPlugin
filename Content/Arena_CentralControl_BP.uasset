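; Central control actor for the ARK Arena mod that performs server-side match-world setup and routes script commands.
; One second after BeginPlay it clears leftover player pawns outside the editor and all enemies, initializes queues and enforces structure safe zones.
; It copies ArkArena INI options into the game mode and game state, then spawns extra singleton classes.
; Game mode custom events are split into command and parameters for HandleScriptCommand.
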(event Custom|OnActorCustomEvent_Event
  (params (EventCustomName :type Name) (EventCustomString :type String) (InstigatorActor :type Actor%20Object%20Reference))
  (bind (_lefts _rights _returnvalue) (Utilities|String|Split EventCustomString " "))
  (if _returnvalue
    (CallFunction|HandleScriptCommand InstigatorActor _lefts _rights)
    (else
      (CallFunction|HandleScriptCommand InstigatorActor EventCustomString))))

(event EventBeginPlay
  (bind _returnvalue (Game|GetGameMode))
  (bind _returnvalue_2 (Game|GetGameState))
  (bind _asshooter_game_state_arena_mod (Utilities|Casting|CastToShooterGameState_ArenaMod _returnvalue_2))
  (Utilities|FlowControl|Delay 0 1.0)
  (if (Networking|IsServer)
    (Utilities|FlowControl|Sequence
      (:then_0
        (bind _astest_game_mode_arena_mod (Utilities|Casting|CastToTestGameMode_ArenaMod _returnvalue))
        (Utilities|FlowControl|Sequence
          (:then_0
            (bind _outactors (Actor|GetAllActorsOfClass 0 "/ArenaMod/PlayerPawnTest_Child_ArenaMod.PlayerPawnTest_Child_ArenaMod_C"))
            (for _array_element _outactors
              (bind _asplayer_pawn_test_child_arena_mod (Utilities|Casting|CastToPlayerPawnTest_Child_ArenaMod _array_element))
              (if (not (Class|VictoryCore|IsEditor))
                (Actor|DestroyActor _asplayer_pawn_test_child_arena_mod))))
          (:then_1
            (Default|InitializeQueues _astest_game_mode_arena_mod))
          (:then_2
            (bind _returnvalue_3 (Class|ShooterGameMode|GetFloatOptionIni _astest_game_mode_arena_mod "ArkArena" "ElementShardsMultiplier"))
            (Variables|/ArenaMod/TestGameMode_ArenaMod.TestGameMode_ArenaMod_C|SetShardsMultiplier _astest_game_mode_arena_mod (Math|Float|Max(Float) _returnvalue_3 1.0)))
          (:then_3
            (EventDispatchers|AssignOnActorCustomEvent _returnvalue (delegate Custom|OnActorCustomEvent_Event)))
          (:then_4
            (bind _returnvalue_4 (Class|ShooterGameMode|GetBoolOptionIni _astest_game_mode_arena_mod "ArkArena" "DisableGold" false))
            (Variables|/ArenaMod/ShooterGameState_ArenaMod.ShooterGameState_ArenaMod_C|SetDisableGold _asshooter_game_state_arena_mod _returnvalue_4 false))
          (:then_5
            (bind _returnvalue_5 (Class|ShooterGameMode|GetFloatOptionIni _astest_game_mode_arena_mod "ArkArena" "AFKTimeout"))
            (Variables|/ArenaMod/ShooterGameState_ArenaMod.ShooterGameState_ArenaMod_C|SetIdleTimeout _asshooter_game_state_arena_mod _returnvalue_5))
          (:then_6
            (bind _returnvalue_6 (Class|ShooterGameMode|GetBoolOptionIni _astest_game_mode_arena_mod "ArkArena" "ForceNameValidation" false))
            (Variables|/ArenaMod/ShooterGameState_ArenaMod.ShooterGameState_ArenaMod_C|SetForceNameValidation _asshooter_game_state_arena_mod _returnvalue_6))
          (:then_7
            (Development|ExecuteConsoleCommand 0 "DestroyAllEnemies" 0))
          (:then_8
            (bind _returnvalue_7 (Class|ShooterGameMode|GetFloatOptionIni _astest_game_mode_arena_mod "ArkArena" "StoreCostMultiplierShards"))
            (Variables|/ArenaMod/ShooterGameState_ArenaMod.ShooterGameState_ArenaMod_C|SetStoreCostMultiplierShards _asshooter_game_state_arena_mod (Math|Float|SelectFloat _returnvalue_7 1.0 (> _returnvalue_7 0.0))))
          (:then_9
            (bind _returnvalue_8 (Class|ShooterGameMode|GetFloatOptionIni _astest_game_mode_arena_mod "ArkArena" "StoreCostMultiplierGold"))
            (Variables|/ArenaMod/ShooterGameState_ArenaMod.ShooterGameState_ArenaMod_C|SetStoreCostMultiplierGold _asshooter_game_state_arena_mod (Math|Float|SelectFloat _returnvalue_8 1.0 (> _returnvalue_8 0.0))))
          (:then_10
            (Default|EnforceStructureSafeZones _astest_game_mode_arena_mod))
          (:then_11
            (for _array_element_2 (Variables|Default|GetExtraSingletonClasses)
              (bind _returnvalue_9 (Class|VictoryCore|BPLoadClass _array_element_2))
              (if (!= _returnvalue_9 0)
                (bind _asactor (Utilities|Casting|CastToActorClass _returnvalue_9))
                (Game|SpawnActorfromClass _asactor (Math|Transform|MakeTransform "0, 0, 0") "AdjustIfPossibleButDontSpawnIfColliding" "SelectDefaultAtRuntime" 0 0)))))))))

(fn ConstructionScript)