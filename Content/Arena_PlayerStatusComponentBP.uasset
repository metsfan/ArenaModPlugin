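; Player status component for the Arena mode that lets a player's level be set directly while blocking other experience gain.
; SetCurrentLevel reads the player experience ramp for the target level, then grants a quarter of the shortfall as unshared generic XP.
; It lifts NeverAllowXP only for that grant and re-enables it afterward.
; The max level and max experience hooks return their inputs unchanged.
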(fn BPModifyMaxLevel
  (params (InMaxLevel :type Integer))
  (return InMaxLevel))

(fn BPModifyMaxExperiencePoints
  (params (InMaxExperiencePoints :type Float%20%28single-precision%29))
  (return InMaxExperiencePoints))

(fn SetCurrentLevel
  (params (Level :type Integer))
  (if (> Level 1)
    (bind _returnvalue (Class|PrimalGameData|BPGetGameData))
    (Variables|Default|SetbNeverAllowXP false)
    (Class|PrimalCharacterStatusComponent|AddExperience (* (- (Utilities|Array|Get(acopy) (Utilities|Struct|BreakLevelExperienceRamp (Class|PrimalGameData|GetLevelExperienceRamp _returnvalue "Player")) (- Level 2)) (Variables|Default|GetExperiencePoints)) 0.25) false "XP_GENERIC")
    (Variables|Default|SetbNeverAllowXP true)))